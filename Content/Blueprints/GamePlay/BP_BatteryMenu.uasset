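; Battery actor, apparently a menu variant of a drone battery, that tracks a clamped charge level and shows it on a WBP_Charge widget.
; Use and Recharge adjust the charge and refresh the widget through ChangeParameters, with a latch so empty updates only once.
; EnginesUsage and ShieldUsage compute draw from the owning BP_DroneBase's thrusters and shield, but nothing here applies it.
; Charge-based color changes and zero-charge drone shutdown are disconnected and never run.
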(event EventBeginPlay
  (CallFunction|Use 0.0))

(event Collision|EventActorBeginOverlap
  (params (OtherActor :type Actor%20Object%20Reference)))

(event EventTick
  (params (DeltaSeconds :type Float%20%28single-precision%29)))

(fn ConstructionScript)

(fn Use
  (params (Power :type Float%20%28double-precision%29))
  (bind _output_get (Variables|Default|SetCharge (Math|Float|Clamp(Float) (- (Variables|Default|GetCharge) Power) 0.0 1e+02)))
  (CallFunction|ChangeParameters _output_get))

(fn Recharge
  (params (Power :type Float%20%28double-precision%29))
  (bind _output_get (Variables|Default|SetCharge (Math|Float|Clamp(Float) (+ (Variables|Default|GetCharge) Power) 0.0 1e+02)))
  (CallFunction|ChangeParameters _output_get))

(fn EnginesUsage
  (bind _asbp_drone_base (Utilities|Casting|CastToBP_DroneBase (Components|GetOwner)))
  (return (* (+ (Variables|/Script/Engine.PhysicsThrusterComponent|GetThrustStrength (Variables|/Script/DroneStabilization.DroneBase|GetPhysicsThrusterBL _asbp_drone_base)) (Variables|/Script/Engine.PhysicsThrusterComponent|GetThrustStrength (Variables|/Script/DroneStabilization.DroneBase|GetPhysicsThrusterBR _asbp_drone_base)) (Variables|/Script/Engine.PhysicsThrusterComponent|GetThrustStrength (Variables|/Script/DroneStabilization.DroneBase|GetPhysicsThrusterFL _asbp_drone_base)) (Variables|/Script/Engine.PhysicsThrusterComponent|GetThrustStrength (Variables|/Script/DroneStabilization.DroneBase|GetPhysicsThrusterFR _asbp_drone_base))) (Variables|Default|GetEnginesMultiplier))))

(fn ChangeParameters
  (params (Charge :type Float%20%28double-precision%29))
  (if (== Charge 0.0)
    (if (not (Variables|Default|GetDisabledAll))
      (Variables|Default|SetDisabledAll true)
      (bind _aswbp_charge (Utilities|Casting|CastToWBP_Charge (UserInterface|GetWidget (Variables|Default|GetWidget)) :!label _label))
      (Default|SetChargeNumber _aswbp_charge Charge))
    (else
      (Utilities|FlowControl|Sequence
        (:then_0
          (Variables|Default|SetDisabledAll false))
        (:then_1
          (goto _label))))))

(fn ShieldUsage
  (bind _asbp_drone_base (Utilities|Casting|CastToBP_DroneBase (Components|GetOwner)))
  (if (Variables|/Game/Drone/Shield/BP_ShieldBase.BP_ShieldBase_C|GetbIsActive (Default|GetShield _asbp_drone_base))
    (return (Variables|Default|GetShieldMultiplier))
    (else
      (return 0.0))))