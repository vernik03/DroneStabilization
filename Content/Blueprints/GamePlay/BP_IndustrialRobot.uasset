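; Industrial robot actor that plays a looping left or right skeletal mesh animation, chosen by the LeftRight flag.
; BeginPlay mutes its audio component and starts the animation.
; When a component tagged AssemblyLineComponent begins overlapping the Box, the same play call runs again.
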(event OnComponentBeginOverlap(Box)
  (params (OverlappedComponent :type Primitive%20Component%20Object%20Reference) (OtherActor :type Actor%20Object%20Reference) (OtherComp :type Primitive%20Component%20Object%20Reference) (OtherBodyIndex :type Integer) (bFromSweep :type Boolean) (SweepResult :type Hit%20Result%20Structure%20%28by%20ref%29))
  (if (>= (Utilities|Array|FindItem (Variables|/Script/Engine.ActorComponent|GetComponentTags OtherComp) "AssemblyLineComponent") 0)
    (Components|Animation|PlayAnimation (Variables|Default|GetIndustrialRobot) (select (Variables|Default|GetLeft\Right) "/Game/Meshes/RobotLarge/SK_IndustrialRobot_Right_Anim.SK_IndustrialRobot_Right_Anim" "/Game/Meshes/RobotLarge/SK_IndustrialRobot_Left_Anim.SK_IndustrialRobot_Left_Anim") true)))

(event EventBeginPlay
  (Audio|Components|Audio|SetVolumeMultiplier (Variables|Default|GetAudio) 0.0 :!class /Script/Engine.AudioComponent)
  (Components|Animation|PlayAnimation (Variables|Default|GetIndustrialRobot) (select (Variables|Default|GetLeft\Right) "/Game/Meshes/RobotLarge/SK_IndustrialRobot_Right_Anim.SK_IndustrialRobot_Right_Anim" "/Game/Meshes/RobotLarge/SK_IndustrialRobot_Left_Anim.SK_IndustrialRobot_Left_Anim") true))

(event Collision|EventActorBeginOverlap
  (params (OtherActor :type Actor%20Object%20Reference)))

(event EventTick
  (params (DeltaSeconds :type Float%20%28single-precision%29)))

(fn ConstructionScript)