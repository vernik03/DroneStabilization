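; BP_ShieldMenu toggles a Niagara shield effect on and off at a regular interval, apparently as a drone shield display for the menu.
; The NSShieldSkeletalDrone effect is deactivated on BeginPlay.
; Tick accumulates time and, each time it reaches Delay, resets the counter and flips IsActive to activate or deactivate the effect.
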(event EventBeginPlay
  (Components|Activation|Deactivate (Variables|Components|GetNS_Shield_Skeletal_Drone)))

(event EventTick
  (params (DeltaSeconds :type Float%20%28single-precision%29))
  (bind _ns_shield_skeletal_drone (Variables|Components|GetNS_Shield_Skeletal_Drone))
  (Variables|Default|Settime (+ DeltaSeconds (Variables|Default|Gettime)))
  (if (>= (Variables|Default|Gettime) (Variables|Default|Getdelay))
    (Variables|Default|Settime 0.0)
    (if (Variables|Default|GetbIsActive)
      (Variables|Default|SetbIsActive false)
      (Components|Activation|Deactivate _ns_shield_skeletal_drone)
      (else
        (Variables|Default|SetbIsActive true)
        (Components|Activation|Activate _ns_shield_skeletal_drone false)))))

(fn ConstructionScript)