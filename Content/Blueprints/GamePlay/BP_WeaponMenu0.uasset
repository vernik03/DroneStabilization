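; Menu weapon actor that animates a weapon mesh along a spline, automatically alternating between activated and deactivated states on a Tick timer.
; A timeline plays forward or reverses to slide the mesh along MainWeaponSpline, deriving roll from spline pitch.
; The timeline also drives Aiming and eases Rotation to zero, while ChangeAiming and ChangeRotation apply clamped offsets to them.
; SetSpline stores a separate Spline variable that the movement ignores.
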(event Custom|DeactivateEvent
  (bind _mainweaponspline (Variables|Default|GetMainWeaponSpline))
  (bind _weaponmesh (Variables|Default|GetWeaponMesh))
  (bind _relativerotation (Variables|/Script/Engine.SceneComponent|GetRelativeRotation _weaponmesh))
  (Variables|Default|SetbIsActivated false)
  (bind (_direction _movement _rotation) (Timeline|Timeline Reverse)
    (:Update
      (Utilities|FlowControl|Sequence
        (:then_0
          (Utilities|IsValid _mainweaponspline
            (:Is%20Valid
              (Transformation|SetRelativeLocationAndRotation _weaponmesh (.location (Spline|GetTransformatDistanceAlongSpline _mainweaponspline (Math|Float|Lerp 0.0 (Spline|GetSplineLength _mainweaponspline) _movement) "Local" false)) (Math|Rotator|MakeRotator (+ (* (.pitch (.rotation (Spline|GetTransformatDistanceAlongSpline _mainweaponspline (Math|Float|Lerp 0.0 (Spline|GetSplineLength _mainweaponspline) _movement) "Local" false))) -1.0) 1.8e+02) (.pitch _relativerotation) (.yaw _relativerotation)) true false))))
        (:then_1
          (Variables|Default|SetAiming _rotation)
          (Variables|Default|SetRotation (Math|Float|Lerp (Variables|Default|GetRotation) 0.0 _movement)))))))

(event Custom|ActivateEvent
  (bind _mainweaponspline (Variables|Default|GetMainWeaponSpline))
  (bind _weaponmesh (Variables|Default|GetWeaponMesh))
  (bind _relativerotation (Variables|/Script/Engine.SceneComponent|GetRelativeRotation _weaponmesh))
  (Variables|Default|SetbIsActivated true)
  (bind (_direction _movement _rotation) (Timeline|Timeline Play)
    (:Update
      (Utilities|FlowControl|Sequence
        (:then_0
          (Utilities|IsValid _mainweaponspline
            (:Is%20Valid
              (Transformation|SetRelativeLocationAndRotation _weaponmesh (.location (Spline|GetTransformatDistanceAlongSpline _mainweaponspline (Math|Float|Lerp 0.0 (Spline|GetSplineLength _mainweaponspline) _movement) "Local" false)) (Math|Rotator|MakeRotator (+ (* (.pitch (.rotation (Spline|GetTransformatDistanceAlongSpline _mainweaponspline (Math|Float|Lerp 0.0 (Spline|GetSplineLength _mainweaponspline) _movement) "Local" false))) -1.0) 1.8e+02) (.pitch _relativerotation) (.yaw _relativerotation)) true false))))
        (:then_1
          (Variables|Default|SetAiming _rotation)
          (Variables|Default|SetRotation (Math|Float|Lerp (Variables|Default|GetRotation) 0.0 _movement)))))))

(event EventBeginPlay
  (Utilities|FlowControl|Delay 0.5)
  (CallFunction|DeactivateEvent))

(event EventTick
  (params (DeltaSeconds :type Float%20%28single-precision%29))
  (Variables|Default|Settime (+ DeltaSeconds (Variables|Default|Gettime)))
  (if (>= (Variables|Default|Gettime) (Variables|Default|Getdelay))
    (Variables|Default|Settime 0.0)
    (if (Variables|Default|GetbIsActivated)
      (CallFunction|DeactivateEvent)
      (else
        (CallFunction|ActivateEvent)))))

(fn ConstructionScript)

(fn SetSpline
  (params (Spline :type Spline%20Component%20Object%20Reference))
  (Variables|Default|SetSpline Spline))

(fn ChangeAiming
  (params (Value :type Float%20%28double-precision%29))
  (Variables|Default|SetAiming (Math|Float|Clamp(Float) (+ (* Value -0.8) (Variables|Default|GetAiming)) -35.0 3e+01)))

(fn ChangeRotation
  (params (Value :type Float%20%28double-precision%29))
  (Variables|Default|SetRotation (Math|Float|Clamp(Float) (+ (* Value 1e+01) (Variables|Default|GetRotation)) -1e+02 1e+02)))