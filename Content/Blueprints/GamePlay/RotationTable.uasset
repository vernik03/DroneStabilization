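; RotationTable is a display actor that slowly spins a tank mesh and animates four fan bones on a poseable mesh.
; Tick turns the tank's relative yaw at a steady, delta-time-scaled rate.
; A Timeline started on BeginPlay sets each fan bone's world-space yaw from its own track, keeping roll and pitch.
; After each run it pauses, then uses the Reverted flag to alternate between forward and reverse playback.
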(event EventBeginPlay
  (bind _poseablemesh (Variables|Default|GetPoseableMesh))
  (bind _poseablemesh_2 (Variables|Default|GetPoseableMesh))
  (bind _poseablemesh_3 (Variables|Default|GetPoseableMesh))
  (bind _poseablemesh_4 (Variables|Default|GetPoseableMesh))
  (bind (_direction _fl _fr _bl _br) (Timeline|Timeline PlayFromStart)
    (:Update
      (Utilities|FlowControl|Sequence
        (:then_0
          (bind _returnvalue (Class|PoseableMeshComponent|GetBoneRotationbyName _poseablemesh_2 "Fan_FL" "WorldSpace"))
          (Components|PoseableMesh|SetBoneRotationbyName _poseablemesh_2 "Fan_FL" (Math|Rotator|MakeRotator (.roll _returnvalue) (.pitch _returnvalue) _fl) "WorldSpace"))
        (:then_1
          (bind _returnvalue_2 (Class|PoseableMeshComponent|GetBoneRotationbyName _poseablemesh_3 "Fan_FR" "WorldSpace"))
          (Components|PoseableMesh|SetBoneRotationbyName _poseablemesh_3 "Fan_FR" (Math|Rotator|MakeRotator (.roll _returnvalue_2) (.pitch _returnvalue_2) _fr) "WorldSpace"))
        (:then_2
          (bind _returnvalue_3 (Class|PoseableMeshComponent|GetBoneRotationbyName _poseablemesh_4 "Fan_BL" "WorldSpace"))
          (Components|PoseableMesh|SetBoneRotationbyName _poseablemesh_4 "Fan_BL" (Math|Rotator|MakeRotator (.roll _returnvalue_3) (.pitch _returnvalue_3) _bl) "WorldSpace"))
        (:then_3
          (bind _returnvalue_4 (Class|PoseableMeshComponent|GetBoneRotationbyName _poseablemesh "Fan_BR" "WorldSpace"))
          (Components|PoseableMesh|SetBoneRotationbyName _poseablemesh "Fan_BR" (Math|Rotator|MakeRotator (.roll _returnvalue_4) (.pitch _returnvalue_4) _br) "WorldSpace"))))
    (:Finished
      (Utilities|FlowControl|Delay 3.0)
      (if (Variables|Default|Getreverted)
        (Variables|Default|Setreverted false)
        (Timeline|Timeline ReverseFromEnd)
        (else
          (Variables|Default|Setreverted true)
          (Timeline|Timeline PlayFromStart))))))

(event Collision|EventActorBeginOverlap
  (params (OtherActor :type Actor%20Object%20Reference)))

(event EventTick
  (params (DeltaSeconds :type Float%20%28single-precision%29))
  (bind _sm_wvc_tank_a (Variables|Default|GetSM_WVC_Tank_A))
  (Transformation|SetRelativeRotation _sm_wvc_tank_a (Math|Rotator|MakeRotator 0.0 0.0 (+ (* DeltaSeconds -6.5) (.yaw (Variables|/Script/Engine.SceneComponent|GetRelativeRotation _sm_wvc_tank_a)))) false false))

(fn ConstructionScript)