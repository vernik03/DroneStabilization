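; BP_Wind is a wind zone actor that pushes drones inside its box volume.
; Each tick it finds overlapping BP_DroneBase actors and applies its Impulse vector to their DroneMesh.
; The impulse is mass-dependent and repeats every frame without delta-time scaling, so the push varies with frame rate.
; It also draws the box as a debug outline every tick.
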(event EventBeginPlay)

(event Collision|EventActorBeginOverlap
  (params (OtherActor :type Actor%20Object%20Reference)))

(event EventTick
  (params (DeltaSeconds :type Float%20%28single-precision%29))
  (bind _box (Variables|Default|GetBox))
  (Rendering|Debug|DrawDebugBox (Transformation|GetWorldLocation _box) (Components|Box|GetScaledBoxExtent _box) "(R=0.000000,G=1.000000,B=0.811689,A=1.000000)" "0, 0, 0" 0.0 3.0)
  (for _array_element (Collision|GetOverlappingActors (Variables|Default|GetBox) "/Game/Drone/BP_DroneBase.BP_DroneBase_C" :!class /Script/Engine.PrimitiveComponent)
    (bind _asbp_drone_base (Utilities|Casting|CastToBP_DroneBase _array_element))
    (Physics|AddImpulse (Variables|/Script/DroneStabilization.DroneBase|GetDroneMesh _asbp_drone_base) (Variables|Default|GetImpulse) "None" false)))

(fn ConstructionScript)