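; Energy generator that recharges the battery of drones passing through its box trigger.
; A drone's skeletal mesh entering triggers one multicast recharge, scaled by a multiplier and the square of its summed absolute velocity components, so faster passes give more charge.
; The ChargingDrones array blocks repeat charges until the overlap ends; gradual recharge logic is left disconnected.
; The construction script snaps the root to whatever surface a forward trace from Tracer hits.
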(event OnComponentBeginOverlap(Box)
  (params (OverlappedComponent :type Primitive%20Component%20Object%20Reference) (OtherActor :type Actor%20Object%20Reference) (OtherComp :type Primitive%20Component%20Object%20Reference) (OtherBodyIndex :type Integer) (bFromSweep :type Boolean) (SweepResult :type Hit%20Result%20Structure%20%28by%20ref%29))
  (bind _chargingdrones (Variables|Default|GetChargingDrones))
  (bind _asskeletal_mesh_component (Utilities|Casting|CastToSkeletalMeshComponent OtherComp))
  (bind _asbp_drone_base (Utilities|Casting|CastToBP_DroneBase OtherActor))
  (if (== (Utilities|Array|FindItem _chargingdrones _asbp_drone_base) -1)
    (Default|MulticastResharge (Default|GetBattery _asbp_drone_base) (* (Variables|Default|GetPoserMultiplier) (Math|Float|Power (+ (.x (Math|Vector|VectorGetAbs (Transformation|GetVelocity _asbp_drone_base))) (.y (Math|Vector|VectorGetAbs (Transformation|GetVelocity _asbp_drone_base))) (.z (Math|Vector|VectorGetAbs (Transformation|GetVelocity _asbp_drone_base)))) 2.0)))
    (Utilities|Array|AddUnique _chargingdrones _asbp_drone_base)))

(event OnComponentEndOverlap(Box)
  (params (OverlappedComponent :type Primitive%20Component%20Object%20Reference) (OtherActor :type Actor%20Object%20Reference) (OtherComp :type Primitive%20Component%20Object%20Reference) (OtherBodyIndex :type Integer))
  (bind _asskeletal_mesh_component (Utilities|Casting|CastToSkeletalMeshComponent OtherComp))
  (bind _asbp_drone_base (Utilities|Casting|CastToBP_DroneBase OtherActor))
  (Utilities|Array|RemoveItem (Variables|Default|GetChargingDrones) _asbp_drone_base))

(event EventBeginPlay)

(event Collision|EventActorBeginOverlap
  (params (OtherActor :type Actor%20Object%20Reference)))

(event EventTick
  (params (DeltaSeconds :type Float%20%28single-precision%29)))

(fn ConstructionScript
  (bind _tracer (Variables|Default|GetTracer))
  (bind _generatrroot (Variables|Default|GetGeneratrRoot))
  (bind _returnvalue (Transformation|GetWorldLocation _tracer))
  (bind _outhit (Collision|LineTraceByChannel _returnvalue (+ _returnvalue (* (Math|Vector|GetForwardVector _tracer) 1e+03)) "TraceTypeQuery2" false 0 "None"))
  (if (.bblockinghit _outhit)
    (Transformation|SetWorldLocation _generatrroot (.location _outhit) false false)
    (else
      (Transformation|SetWorldLocation _generatrroot (Transformation|GetWorldLocation _generatrroot) false false))))