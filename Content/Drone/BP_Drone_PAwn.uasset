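; Physics-driven quadcopter pawn, flown with Enhanced Input and registerable with a Learning Agents manager when IsAgent is set.
; Throttle, pitch, roll and yaw inputs accumulate per-rotor power, which Tick adds to base thruster thrust, mirrors in fan torque and rumble, then clears.
; Inputs override StabilizationComponent axes, easing off at higher tilt.
; Box overlaps fire a hit dispatcher; resetting unbinds it, restores the start position and applies a random impulse.
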(event OnComponentBeginOverlap(Box)
  (params (OverlappedComponent :type Primitive%20Component%20Object%20Reference) (OtherActor :type Actor%20Object%20Reference) (OtherComp :type Primitive%20Component%20Object%20Reference) (OtherBodyIndex :type Integer) (bFromSweep :type Boolean) (SweepResult :type Hit%20Result%20Structure%20%28by%20ref%29))
  (Default|CallHitEventDispatcher OtherActor self))

(event Custom|RegisterAgents
  (bind _outactors (Actor|GetAllActorswithTag "LearningAgentsManager"))
  (for _array_element _outactors
    (Utilities|IsValid (Actor|GetComponentbyClass _array_element "/Script/LearningAgents.LearningAgentsManager")
      (:Is%20Valid
        (Class|LearningAgentsManager|AddAgent (Actor|GetComponentbyClass _array_element "/Script/LearningAgents.LearningAgentsManager") self)
        (Variables|Default|SetFoundManager true))))
  (if (not (Variables|Default|GetFoundManager))
    (Development|PrintString "Could not find Learning Agents manager. Did we forget to add one to the scene?")))

(event Input|EnhancedActionEvents|EnhancedInputActionIA_FL
  (params (ActionValue :type Boolean) (ElapsedSeconds :type Float%20%28double-precision%29) (TriggeredSeconds :type Float%20%28double-precision%29) (InputAction :type Input%20Action%20Object%20Reference :default "/Game/Drone/Input/IA_FL.IA_FL"))
  (bind _physicsthrusterfl (Variables|Default|GetPhysicsThrusterFL))
  (:Started
    (Components|Activation|SetActive _physicsthrusterfl true true)
    (Variables|/Script/Engine.PhysicsThrusterComponent|SetThrustStrength _physicsthrusterfl (Variables|Default|GetThrust%20Strength%20Base)))
  (:Completed
    (Components|Activation|SetActive _physicsthrusterfl false true)
    (Variables|/Script/Engine.PhysicsThrusterComponent|SetThrustStrength _physicsthrusterfl 0.0)))

(event Input|EnhancedActionEvents|EnhancedInputActionIA_FR
  (params (ActionValue :type Boolean) (ElapsedSeconds :type Float%20%28double-precision%29) (TriggeredSeconds :type Float%20%28double-precision%29) (InputAction :type Input%20Action%20Object%20Reference :default "/Game/Drone/Input/IA_FR.IA_FR"))
  (bind _physicsthrusterfr (Variables|Default|GetPhysicsThrusterFR))
  (:Started
    (Components|Activation|SetActive _physicsthrusterfr true true)
    (Variables|/Script/Engine.PhysicsThrusterComponent|SetThrustStrength _physicsthrusterfr (Variables|Default|GetThrust%20Strength%20Base)))
  (:Completed
    (Components|Activation|SetActive _physicsthrusterfr false true)
    (Variables|/Script/Engine.PhysicsThrusterComponent|SetThrustStrength _physicsthrusterfr 0.0)))

(event Input|EnhancedActionEvents|EnhancedInputActionIA_ChangeCamera
  (params (ActionValue :type Boolean) (ElapsedSeconds :type Float%20%28double-precision%29) (TriggeredSeconds :type Float%20%28double-precision%29) (InputAction :type Input%20Action%20Object%20Reference :default "/Game/Drone/Input/IA_ChangeCamera.IA_ChangeCamera"))
  (:Started
    (Components|Activation|SetActive (Variables|Default|GetTopCamera) true false)
    (Components|Activation|SetActive (Variables|Default|GetCamera) false false))
  (:Completed
    (Components|Activation|SetActive (Variables|Default|GetTopCamera) false false)
    (Components|Activation|SetActive (Variables|Default|GetCamera) true false)))

(event Input|EnhancedActionEvents|EnhancedInputActionIA_Stabilize
  (params (ActionValue :type Boolean) (ElapsedSeconds :type Float%20%28double-precision%29) (TriggeredSeconds :type Float%20%28double-precision%29) (InputAction :type Input%20Action%20Object%20Reference :default "/Game/Drone/Input/IA_Stabilize.IA_Stabilize"))
  (bind _material (Variables|Default|GetMaterial))
  (:Started
    (if (Variables|Default|GetIsStabilization)
      (Variables|Default|SetIsStabilization false)
      (Rendering|Material|SetVectorParameterValue _material "LightColor" "(R=1.000000,G=1.000000,B=1.000000,A=0.000000)" :!class /Script/Engine.MaterialInstanceDynamic)
      (else
        (Variables|Default|SetIsStabilization true)
        (Rendering|Material|SetVectorParameterValue _material "LightColor" "(R=0.000000,G=1.000000,B=0.294245,A=1.000000)" :!class /Script/Engine.MaterialInstanceDynamic)))))

(event Input|EnhancedActionEvents|EnhancedInputActionIA_InputSettings
  (params (ActionValue :type Boolean) (ElapsedSeconds :type Float%20%28double-precision%29) (TriggeredSeconds :type Float%20%28double-precision%29) (InputAction :type Input%20Action%20Object%20Reference :default "/Game/Drone/Input/IA_InputSettings.IA_InputSettings"))
  (:Started
    (if (Variables|Default|GetIsSettingsActive)
      (Variables|Default|SetIsSettingsActive false)
      (else
        (Variables|Default|SetIsSettingsActive true)))))

(event Input|EnhancedActionEvents|EnhancedInputActionIA_PowerAll
  (params (ActionValue :type Float%20%28double-precision%29) (ElapsedSeconds :type Float%20%28double-precision%29) (TriggeredSeconds :type Float%20%28double-precision%29) (InputAction :type Input%20Action%20Object%20Reference :default "/Game/Drone/Input/IA_PowerAll.IA_PowerAll"))
  (bind _returnvalue (* ActionValue 4e+02))
  (bind _stabilizationcomponent (Variables|Default|GetStabilizationComponent))
  (bind _thrust_strength_base (Variables|Default|GetThrust%20Strength%20Base))
  (bind _returnvalue_2 (* _thrust_strength_base -1.0))
  (:Triggered
    (Variables|/Game/Drone/StabilizationComponent.StabilizationComponent_C|SetHeightVelocityDeactivate _stabilizationcomponent true)
    (Utilities|FlowControl|Sequence
      (:then_0
        (Variables|Default|SetFR_TickPower (Math|Float|Clamp(Float) (+ (Variables|Default|GetFR_TickPower) _returnvalue) _returnvalue_2 1e+04)))
      (:then_1
        (Variables|Default|SetFL_TickPower (Math|Float|Clamp(Float) (+ (Variables|Default|GetFL_TickPower) _returnvalue) _returnvalue_2 1e+04)))
      (:then_2
        (Variables|Default|SetBL_TickPower (Math|Float|Clamp(Float) (+ (Variables|Default|GetBL_TickPower) _returnvalue) _returnvalue_2 1e+04)))
      (:then_3
        (Variables|Default|SetBR_TickPower (Math|Float|Clamp(Float) (+ (Variables|Default|GetBR_TickPower) _returnvalue) _returnvalue_2 1e+04)))))
  (:Completed
    (Variables|/Game/Drone/StabilizationComponent.StabilizationComponent_C|SetHeightVelocityDeactivate _stabilizationcomponent false)))

(event Input|EnhancedActionEvents|EnhancedInputActionIA_Rotate
  (params (ActionValue :type Float%20%28double-precision%29) (ElapsedSeconds :type Float%20%28double-precision%29) (TriggeredSeconds :type Float%20%28double-precision%29) (InputAction :type Input%20Action%20Object%20Reference :default "/Game/Drone/Input/IA_Rotate.IA_Rotate"))
  (bind _stabilizationcomponent (Variables|Default|GetStabilizationComponent))
  (bind _deltapower (Variables|Default|GetDeltaPower))
  (bind _deltapower_2 (Variables|Default|GetDeltaPower))
  (bind _deltapower_3 (Variables|Default|GetDeltaPower))
  (bind _deltapower_4 (Variables|Default|GetDeltaPower))
  (bind _returnvalue (* _deltapower_2 -1.0))
  (bind _returnvalue_2 (* ActionValue _deltapower_3))
  (bind _returnvalue_3 (* ActionValue _deltapower))
  (bind _returnvalue_4 (* _deltapower_4 -1.0))
  (bind _returnvalue_5 (* ActionValue _returnvalue))
  (bind _returnvalue_6 (* ActionValue _returnvalue_4))
  (:Triggered
    (Variables|/Game/Drone/StabilizationComponent.StabilizationComponent_C|SetHorizontalRotationDeactivate _stabilizationcomponent true)
    (if (>= ActionValue 0.0)
      (Utilities|FlowControl|Sequence
        (:then_0
          (Variables|Default|SetFR_TickPower (+ (Variables|Default|GetFR_TickPower) _returnvalue_5)))
        (:then_1
          (Variables|Default|SetFL_TickPower (+ (Variables|Default|GetFL_TickPower) _returnvalue_2)))
        (:then_2
          (Variables|Default|SetBL_TickPower (+ (Variables|Default|GetBL_TickPower) _returnvalue_5)))
        (:then_3
          (Variables|Default|SetBR_TickPower (+ (Variables|Default|GetBR_TickPower) _returnvalue_2))))
      (else
        (Utilities|FlowControl|Sequence
          (:then_0
            (Variables|Default|SetFR_TickPower (+ (Variables|Default|GetFR_TickPower) _returnvalue_6)))
          (:then_1
            (Variables|Default|SetFL_TickPower (+ (Variables|Default|GetFL_TickPower) _returnvalue_3)))
          (:then_2
            (Variables|Default|SetBL_TickPower (+ (Variables|Default|GetBL_TickPower) _returnvalue_6)))
          (:then_3
            (Variables|Default|SetBR_TickPower (+ (Variables|Default|GetBR_TickPower) _returnvalue_3)))))))
  (:Completed
    (Variables|/Game/Drone/StabilizationComponent.StabilizationComponent_C|SetHorizontalRotationDeactivate _stabilizationcomponent false)))

(event Input|EnhancedActionEvents|EnhancedInputActionIA_BL
  (params (ActionValue :type Boolean) (ElapsedSeconds :type Float%20%28double-precision%29) (TriggeredSeconds :type Float%20%28double-precision%29) (InputAction :type Input%20Action%20Object%20Reference :default "/Game/Drone/Input/IA_BL.IA_BL"))
  (bind _physicsthrusterbl (Variables|Default|GetPhysicsThrusterBL))
  (:Started
    (Components|Activation|SetActive _physicsthrusterbl true false)
    (Variables|/Script/Engine.PhysicsThrusterComponent|SetThrustStrength _physicsthrusterbl (Variables|Default|GetThrust%20Strength%20Base)))
  (:Completed
    (Components|Activation|SetActive _physicsthrusterbl false false)
    (Variables|/Script/Engine.PhysicsThrusterComponent|SetThrustStrength _physicsthrusterbl 0.0)))

(event Input|EnhancedActionEvents|EnhancedInputActionIA_BR
  (params (ActionValue :type Boolean) (ElapsedSeconds :type Float%20%28double-precision%29) (TriggeredSeconds :type Float%20%28double-precision%29) (InputAction :type Input%20Action%20Object%20Reference :default "/Game/Drone/Input/IA_BR.IA_BR"))
  (bind _physicsthrusterbr (Variables|Default|GetPhysicsThrusterBR))
  (:Started
    (Components|Activation|SetActive _physicsthrusterbr true false)
    (Variables|/Script/Engine.PhysicsThrusterComponent|SetThrustStrength _physicsthrusterbr (Variables|Default|GetThrust%20Strength%20Base)))
  (:Completed
    (Components|Activation|SetActive _physicsthrusterbr false false)
    (Variables|/Script/Engine.PhysicsThrusterComponent|SetThrustStrength _physicsthrusterbr 0.0)))

(event Input|EnhancedActionEvents|EnhancedInputActionIA_PowerON
  (params (ActionValue :type Boolean) (ElapsedSeconds :type Float%20%28double-precision%29) (TriggeredSeconds :type Float%20%28double-precision%29) (InputAction :type Input%20Action%20Object%20Reference :default "/Game/Drone/Input/IA_PowerON.IA_PowerON"))
  (bind _returnvalue (Game|GetPlayerController 0))
  (:Started
    (if (Variables|Default|GetIsEnginesActivated)
      (Variables|Default|SetIsEnginesActivated false)
      (CallFunction|SetAllActive false)
      (bind _asbp_player_controller (Utilities|Casting|CastToBP_PlayerController _returnvalue))
      (else
        (Variables|Default|SetIsEnginesActivated true)
        (CallFunction|SetAllActive true)
        (bind _asbp_player_controller_2 (Utilities|Casting|CastToBP_PlayerController _returnvalue))))))

(event Input|EnhancedActionEvents|EnhancedInputActionIA_Front_Back
  (params (ActionValue :type Float%20%28double-precision%29) (ElapsedSeconds :type Float%20%28double-precision%29) (TriggeredSeconds :type Float%20%28double-precision%29) (InputAction :type Input%20Action%20Object%20Reference :default "/Game/Drone/Input/IA_Front_Back.IA_Front_Back"))
  (bind _stabilizationcomponent (Variables|Default|GetStabilizationComponent))
  (bind _deltapower (Variables|Default|GetDeltaPower))
  (bind _deltapower_2 (Variables|Default|GetDeltaPower))
  (bind _frontbackmaximumpower (Variables|Default|GetFrontBackMaximumPower))
  (bind _frontbackmaximumpower_2 (Variables|Default|GetFrontBackMaximumPower))
  (bind _returnvalue (* _frontbackmaximumpower_2 -1.0))
  (bind _returnvalue_2 (Math|Float|Clamp(Float) ActionValue _returnvalue _frontbackmaximumpower))
  (bind _returnvalue_3 (* _returnvalue_2 0.0))
  (bind _returnvalue_4 (* _returnvalue_2 _deltapower))
  (bind _returnvalue_5 (* _returnvalue_2 0.0))
  (bind _returnvalue_6 (* _returnvalue_2 _deltapower_2))
  (:Triggered
    (Variables|/Game/Drone/StabilizationComponent.StabilizationComponent_C|SetFrontBackHorizontalDeactivate _stabilizationcomponent true)
    (if (< (Math|Float|Absolute(Float) (.pitch (Transformation|GetActorRotation))) 5.0)
      _
      (else
        (Variables|/Game/Drone/StabilizationComponent.StabilizationComponent_C|SetFrontBackHorizontalLow _stabilizationcomponent true)
        (Variables|/Game/Drone/StabilizationComponent.StabilizationComponent_C|SetFrontBackHorizontalDeactivate _stabilizationcomponent false)))
    (if (>= ActionValue 0.0)
      (Utilities|FlowControl|Sequence
        (:then_0
          (Variables|Default|SetFR_TickPower (+ (Variables|Default|GetFR_TickPower) _returnvalue_6)))
        (:then_1
          (Variables|Default|SetFL_TickPower (+ (Variables|Default|GetFL_TickPower) _returnvalue_6)))
        (:then_2
          (Variables|Default|SetBL_TickPower (+ (Variables|Default|GetBL_TickPower) _returnvalue_5)))
        (:then_3
          (Variables|Default|SetBR_TickPower (+ (Variables|Default|GetBR_TickPower) _returnvalue_5))))
      (else
        (Utilities|FlowControl|Sequence
          (:then_0
            (Variables|Default|SetFR_TickPower (+ (Variables|Default|GetFR_TickPower) _returnvalue_4)))
          (:then_1
            (Variables|Default|SetFL_TickPower (+ (Variables|Default|GetFL_TickPower) _returnvalue_4)))
          (:then_2
            (Variables|Default|SetBL_TickPower (+ (Variables|Default|GetBL_TickPower) _returnvalue_3)))
          (:then_3
            (Variables|Default|SetBR_TickPower (+ (Variables|Default|GetBR_TickPower) _returnvalue_3)))))))
  (:Completed
    (Variables|/Game/Drone/StabilizationComponent.StabilizationComponent_C|SetFrontBackHorizontalDeactivate _stabilizationcomponent false)
    (Variables|/Game/Drone/StabilizationComponent.StabilizationComponent_C|SetFrontBackHorizontalLow _stabilizationcomponent false)))

(event Input|EnhancedActionEvents|EnhancedInputActionIA_Left_Right
  (params (ActionValue :type Float%20%28double-precision%29) (ElapsedSeconds :type Float%20%28double-precision%29) (TriggeredSeconds :type Float%20%28double-precision%29) (InputAction :type Input%20Action%20Object%20Reference :default "/Game/Drone/Input/IA_Left_Right.IA_Left_Right"))
  (bind _stabilizationcomponent (Variables|Default|GetStabilizationComponent))
  (bind _deltapower (Variables|Default|GetDeltaPower))
  (bind _deltapower_2 (Variables|Default|GetDeltaPower))
  (bind _leftrightmaximumpower (Variables|Default|GetLeftRightMaximumPower))
  (bind _leftrightmaximumpower_2 (Variables|Default|GetLeftRightMaximumPower))
  (bind _returnvalue (* _leftrightmaximumpower -1.0))
  (bind _returnvalue_2 (Math|Float|Clamp(Float) ActionValue _returnvalue _leftrightmaximumpower_2))
  (bind _returnvalue_3 (* _returnvalue_2 0.0))
  (bind _returnvalue_4 (* _returnvalue_2 _deltapower))
  (bind _returnvalue_5 (* _returnvalue_2 0.0))
  (bind _returnvalue_6 (* _returnvalue_2 _deltapower_2))
  (:Triggered
    (Variables|/Game/Drone/StabilizationComponent.StabilizationComponent_C|SetLeftRightHorizontalDeactivate _stabilizationcomponent true)
    (if (< (Math|Float|Absolute(Float) (.roll (Transformation|GetActorRotation))) 5.0)
      _
      (else
        (Variables|/Game/Drone/StabilizationComponent.StabilizationComponent_C|SetLeftRightHorizontalLow _stabilizationcomponent true)
        (Variables|/Game/Drone/StabilizationComponent.StabilizationComponent_C|SetLeftRightHorizontalDeactivate _stabilizationcomponent false)))
    (if (>= ActionValue 0.0)
      (Utilities|FlowControl|Sequence
        (:then_0
          (Variables|Default|SetFR_TickPower (+ (Variables|Default|GetFR_TickPower) _returnvalue_5)))
        (:then_1
          (Variables|Default|SetFL_TickPower (+ (Variables|Default|GetFL_TickPower) _returnvalue_6)))
        (:then_2
          (Variables|Default|SetBL_TickPower (+ (Variables|Default|GetBL_TickPower) _returnvalue_6)))
        (:then_3
          (Variables|Default|SetBR_TickPower (+ (Variables|Default|GetBR_TickPower) _returnvalue_5))))
      (else
        (Utilities|FlowControl|Sequence
          (:then_0
            (Variables|Default|SetFR_TickPower (+ (Variables|Default|GetFR_TickPower) _returnvalue_3)))
          (:then_1
            (Variables|Default|SetFL_TickPower (+ (Variables|Default|GetFL_TickPower) _returnvalue_4)))
          (:then_2
            (Variables|Default|SetBL_TickPower (+ (Variables|Default|GetBL_TickPower) _returnvalue_4)))
          (:then_3
            (Variables|Default|SetBR_TickPower (+ (Variables|Default|GetBR_TickPower) _returnvalue_3)))))))
  (:Completed
    (Variables|/Game/Drone/StabilizationComponent.StabilizationComponent_C|SetLeftRightHorizontalDeactivate _stabilizationcomponent false)
    (Variables|/Game/Drone/StabilizationComponent.StabilizationComponent_C|SetLeftRightHorizontalLow _stabilizationcomponent false)))

(event Input|EnhancedActionEvents|EnhancedInputActionIA_Reset
  (params (ActionValue :type Boolean) (ElapsedSeconds :type Float%20%28double-precision%29) (TriggeredSeconds :type Float%20%28double-precision%29) (InputAction :type Input%20Action%20Object%20Reference :default "/Game/VehicleTemplate/Input/Actions/IA_Reset.IA_Reset"))
  (CallFunction|ResettoStartPosition))

(event EventBeginPlay
  (bind _returnvalue (Game|GetPlayerController 0))
  (bind _returnvalue_2 (Game|GetPlayerController 0))
  (bind _skeletalmesh (Variables|Default|GetSkeletalMesh))
  (bind _returnvalue_3 (PlayerController|LocalPlayerSubsystems|GetEnhancedInputLocalPlayerSubsystem _returnvalue))
  (bind _returnvalue_4 (Rendering|Material|CreateDynamicMaterialInstance (Variables|Default|GetSkeletalMesh) 0 "/Game/Materials/M_LampDrone.M_LampDrone" "None" :!class /Script/Engine.PrimitiveComponent))
  (Variables|Default|SetMaterial _returnvalue_4)
  (Variables|Default|SetStartLocation (Transformation|GetActorLocation))
  (if (Variables|Default|GetIsAgent)
    (CallFunction|RegisterAgents)
    (Utilities|FlowControl|Sequence
      (:then_0
        (Class|PrimitiveComponent|SetCenterOfMass _skeletalmesh (Math|Vector|MakeVector (/ (.x (Math|Vector|RotateVector (- (/ (+ (Transformation|GetWorldLocation (Variables|Default|GetPhysicsThrusterFR)) (Transformation|GetWorldLocation (Variables|Default|GetPhysicsThrusterBR))) 2.0) (Physics|GetCenterOfMass _skeletalmesh "None")) (Class|KismetMathLibrary|NegateRotator (Transformation|GetWorldRotation _skeletalmesh)))) 1e+02) 0.0 0.0) "None" :!label _label)
        (Utilities|IsValid _returnvalue_3
          (:Is%20Valid
            (Input|AddMappingContext _returnvalue_3 "/Game/Drone/Input/InputMappingContext.InputMappingContext" 0 "(bIgnoreAllPressedKeysUntilRelease=True,bForceImmediately=False,bNotifyUserSettings=False)"))))
      (:then_1
        (if (Variables|Default|GetIsEnginesActivated)
          (Variables|Default|SetIsEnginesActivated false)
          (CallFunction|SetAllActive false)
          (bind _asbp_player_controller (Utilities|Casting|CastToBP_PlayerController _returnvalue_2))
          (else
            (Variables|Default|SetIsEnginesActivated true)
            (CallFunction|SetAllActive true)
            (bind _asbp_player_controller_2 (Utilities|Casting|CastToBP_PlayerController _returnvalue_2)))))
      (:then_2
        (if (Variables|Default|GetIsStabilization)
          (Variables|Default|SetIsStabilization false)
          (Rendering|Material|SetVectorParameterValue (Variables|Default|GetMaterial) "LightColor" "(R=1.000000,G=1.000000,B=1.000000,A=0.000000)" :!class /Script/Engine.MaterialInstanceDynamic)
          (else
            (Variables|Default|SetIsStabilization true)
            (Rendering|Material|SetVectorParameterValue (Variables|Default|GetMaterial) "LightColor" "(R=0.000000,G=1.000000,B=0.294245,A=1.000000)" :!class /Script/Engine.MaterialInstanceDynamic)))))
    (else
      (goto _label))))

(event EventTick
  (params (DeltaSeconds :type Float%20%28single-precision%29))
  (bind _springarm1 (Variables|Default|GetSpringArm1))
  (bind _skeletalmesh (Variables|Default|GetSkeletalMesh))
  (bind _thrust_strength_base (Variables|Default|GetThrust%20Strength%20Base))
  (bind _thrust_strength_base_2 (Variables|Default|GetThrust%20Strength%20Base))
  (bind __rotationpower (Variables|Default|Get+RotationPower))
  (bind ___rotationpower (Variables|Default|Get++RotationPower))
  (if (Variables|Default|GetIsEnginesActivated)
    (bind _asbp_player_controller (Utilities|Casting|CastToBP_PlayerController (Game|GetPlayerController 0)))
    (Utilities|FlowControl|Sequence
      (:then_0
        (Utilities|FlowControl|Sequence
          (:then_0
            (Utilities|FlowControl|Sequence
              (:then_0
                (bind _output_get (Variables|/Script/Engine.PhysicsThrusterComponent|SetThrustStrength (Variables|Default|GetPhysicsThrusterFR) (+ _thrust_strength_base (Variables|Default|GetFR_TickPower))))
                (Game|Feedback|PlayDynamicForceFeedback _asbp_player_controller (/ _output_get 4e+02) 0.1 false false false true))
              (:then_1
                (bind _output_get_2 (Variables|/Script/Engine.PhysicsThrusterComponent|SetThrustStrength (Variables|Default|GetPhysicsThrusterFL) (+ _thrust_strength_base (Variables|Default|GetFL_TickPower))))
                (Game|Feedback|PlayDynamicForceFeedback _asbp_player_controller (/ _output_get_2 4e+02) 0.1 false true false false))
              (:then_2
                (bind _output_get_3 (Variables|/Script/Engine.PhysicsThrusterComponent|SetThrustStrength (Variables|Default|GetPhysicsThrusterBL) (+ _thrust_strength_base (Variables|Default|GetBL_TickPower))))
                (Game|Feedback|PlayDynamicForceFeedback _asbp_player_controller (/ _output_get_3 4e+02) 0.1 true false false false))
              (:then_3
                (bind _output_get_4 (Variables|/Script/Engine.PhysicsThrusterComponent|SetThrustStrength (Variables|Default|GetPhysicsThrusterBR) (+ _thrust_strength_base (Variables|Default|GetBR_TickPower))))
                (Game|Feedback|PlayDynamicForceFeedback _asbp_player_controller (/ _output_get_4 4e+02) 0.1 false false true false))))
          (:then_1
            (Utilities|FlowControl|Sequence
              (:then_0
                (Class|PrimitiveComponent|AddTorqueinDegrees _skeletalmesh (Math|Vector|MakeVector 0.0 0.0 (* (* (+ (* (Variables|Default|GetBL_TickPower) ___rotationpower) _thrust_strength_base_2) -1.0) __rotationpower)) "Fan_BL_end" true))
              (:then_1
                (Class|PrimitiveComponent|AddTorqueinDegrees _skeletalmesh (Math|Vector|MakeVector 0.0 0.0 (* (+ (* (Variables|Default|GetBR_TickPower) ___rotationpower) _thrust_strength_base_2) __rotationpower)) "Fan_BR_end" true))
              (:then_2
                (Class|PrimitiveComponent|AddTorqueinDegrees _skeletalmesh (Math|Vector|MakeVector 0.0 0.0 (* (* (+ (* (Variables|Default|GetFR_TickPower) ___rotationpower) _thrust_strength_base_2) -1.0) __rotationpower)) "Fan_FR_end" true))
              (:then_3
                (Class|PrimitiveComponent|AddTorqueinDegrees _skeletalmesh (Math|Vector|MakeVector 0.0 0.0 (* (+ (* (Variables|Default|GetFL_TickPower) ___rotationpower) _thrust_strength_base_2) __rotationpower)) "Fan_FL_end" true))
              (:then_4
                (if (Variables|Default|GetIsAgent)
                  _
                  (else
                    _))
                (Utilities|FlowControl|Sequence
                  (:then_0
                    (Variables|Default|SetFR_TickPower 0.0))
                  (:then_1
                    (Variables|Default|SetFL_TickPower 0.0))
                  (:then_2
                    (Variables|Default|SetBL_TickPower 0.0))
                  (:then_3
                    (Variables|Default|SetBR_TickPower 0.0))))))))
      (:then_1
        (Variables|/Script/Engine.SceneComponent|SetbAbsoluteRotation _springarm1 true)
        (Transformation|SetWorldRotation _springarm1 (Math|Rotator|MakeRotator 0.0 -9e+01 (.yaw (Transformation|GetActorRotation))) false false)))))

(fn ConstructionScript)

(fn SetAllActive
  (params (IsActive :type Boolean))
  (bind _physicsthrusterfl (Variables|Default|GetPhysicsThrusterFL))
  (bind _physicsthrusterbl (Variables|Default|GetPhysicsThrusterBL))
  (bind _physicsthrusterbr (Variables|Default|GetPhysicsThrusterBR))
  (bind _physicsthrusterfr (Variables|Default|GetPhysicsThrusterFR))
  (bind _thrust_strength_base (Variables|Default|GetThrust%20Strength%20Base))
  (bind _returnvalue (* _thrust_strength_base IsActive))
  (Utilities|FlowControl|Sequence
    (:then_0
      (Components|Activation|SetActive _physicsthrusterfl IsActive false))
    (:then_1
      (Components|Activation|SetActive _physicsthrusterbl IsActive false))
    (:then_2
      (Components|Activation|SetActive _physicsthrusterbr IsActive false))
    (:then_3
      (Components|Activation|SetActive _physicsthrusterfr IsActive false))
    (:then_4
      (Utilities|FlowControl|Sequence
        (:then_0
          (Variables|/Script/Engine.PhysicsThrusterComponent|SetThrustStrength _physicsthrusterfl _returnvalue))
        (:then_1
          (Variables|/Script/Engine.PhysicsThrusterComponent|SetThrustStrength _physicsthrusterbl _returnvalue))
        (:then_2
          (Variables|/Script/Engine.PhysicsThrusterComponent|SetThrustStrength _physicsthrusterbr _returnvalue))
        (:then_3
          (Variables|/Script/Engine.PhysicsThrusterComponent|SetThrustStrength _physicsthrusterfr _returnvalue))))))

(fn ResettoStartPosition
  (bind _thrust_strength_base (Variables|Default|GetThrust%20Strength%20Base))
  (bind _skeletalmesh (Variables|Default|GetSkeletalMesh))
  (EventDispatchers|UnbindallEventsfromHitEventDispatcher)
  (Physics|SetSimulatePhysics (Variables|Default|GetSkeletalMesh) false)
  (Physics|SetPhysicsLinearVelocity _skeletalmesh "0, 0, 0" false "None")
  (Class|PrimitiveComponent|SetPhysicsAngularVelocityinDegrees _skeletalmesh "0, 0, 0" false "None") ; Interrupt any angular movement
  (Transformation|SetActorLocation (Variables|Default|GetStartLocation) false true)
  (Transformation|SetActorRotation "0, 0, 0" true)
  (Class|SkeletalMeshComponent|ResetAllBodiesSimulatePhysics (Variables|Default|GetSkeletalMesh))
  (Default|ResettoDefaults (Variables|Default|GetStabilizationComponent))
  (Utilities|FlowControl|Sequence
    (:then_0
      (Variables|Default|SetFR_TickPower 0.0)
      (Variables|/Script/Engine.PhysicsThrusterComponent|SetThrustStrength (Variables|Default|GetPhysicsThrusterFR) _thrust_strength_base))
    (:then_1
      (Variables|Default|SetFL_TickPower 0.0)
      (Variables|/Script/Engine.PhysicsThrusterComponent|SetThrustStrength (Variables|Default|GetPhysicsThrusterFL) _thrust_strength_base))
    (:then_2
      (Variables|Default|SetBR_TickPower 0.0)
      (Variables|/Script/Engine.PhysicsThrusterComponent|SetThrustStrength (Variables|Default|GetPhysicsThrusterBL) _thrust_strength_base))
    (:then_3
      (Variables|Default|SetBL_TickPower 0.0)
      (Variables|/Script/Engine.PhysicsThrusterComponent|SetThrustStrength (Variables|Default|GetPhysicsThrusterBR) _thrust_strength_base))
    (:then_4
      (Physics|SetSimulatePhysics (Variables|Default|GetSkeletalMesh) true)
      (CallFunction|AddRandomImpulse))))

(fn AddRandomImpulse
  (Physics|AddImpulse (Variables|Default|GetSkeletalMesh) (Math|Vector|MakeVector 0.0 0.0 (Math|Random|RandomFloatinRange -5e+02 7e+02)) "None" false)
  (Class|PrimitiveComponent|AddTorqueinDegrees (Variables|Default|GetSkeletalMesh) (Math|Vector|MakeVector 0.0 0.0 (Math|Random|RandomFloatinRange -3e+04 3e+04)) "None" true))