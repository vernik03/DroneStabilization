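; Drone battery actor that holds a clamped charge and powers its owning BP_DroneBase.
; Each Tick drains it by thruster strength and active shield cost, without delta-time scaling; shield hits, bound after a startup delay, drain it by impulse.
; Every change updates the charge widget and color-codes battery and drone materials by threshold.
; At empty it goes dark and shuts off drone power and shield once, latched by DisabledAll.
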(event Custom|OnHitEventDispatcher_Event
  (params (Impulse :type Float%20%28double-precision%29))
  (Development|PrintString (Utilities|String|ToString(Float) Impulse))
  (CallFunction|Use (* Impulse (Variables|Default|GetShieldHitMultiplier))))

(event EventBeginPlay
  (bind _returnvalue (Rendering|Material|CreateDynamicMaterialInstance (Variables|Default|GetBatteryMesh) 0 "/Game/Drone/Battery/Mesh/glow.glow" "None" :!class /Script/Engine.PrimitiveComponent))
  (Variables|Default|SetColor _returnvalue)
  (CallFunction|Recharge 0.0)
  (Utilities|FlowControl|Delay 2.0)
  (bind _asbp_drone_base (Utilities|Casting|CastToBP_DroneBase (Components|GetOwner)))
  (EventDispatchers|AssignOnHitEventDispatcher (Default|GetShield _asbp_drone_base) (delegate Custom|OnHitEventDispatcher_Event)))

(event Collision|EventActorBeginOverlap
  (params (OtherActor :type Actor%20Object%20Reference)))

(event EventTick
  (params (DeltaSeconds :type Float%20%28single-precision%29))
  (CallFunction|Use (+ (CallFunction|EnginesUsage) (CallFunction|ShieldUsage))))

(fn ConstructionScript)

(fn Use
  (params (Power :type Float%20%28double-precision%29))
  (bind _output_get (Variables|Default|SetCharge (Math|Float|Clamp(Float) (- (Variables|Default|GetCharge) Power) 0.0 1e+02)))
  (CallFunction|ChangeParameters _output_get))

(fn Recharge
  (params (Power :type Float%20%28double-precision%29))
  (bind _output_get (Variables|Default|SetCharge (Math|Float|Clamp(Float) (+ (Variables|Default|GetCharge) Power) 0.0 1e+02)))
  (CallFunction|ChangeParameters _output_get))

(fn EnginesUsage
  (bind _asbp_drone_base (Utilities|Casting|CastToBP_DroneBase (Components|GetOwner)))
  (return (* (+ (Variables|/Script/Engine.PhysicsThrusterComponent|GetThrustStrength (Variables|/Script/DroneStabilization.DroneBase|GetPhysicsThrusterBL _asbp_drone_base)) (Variables|/Script/Engine.PhysicsThrusterComponent|GetThrustStrength (Variables|/Script/DroneStabilization.DroneBase|GetPhysicsThrusterBR _asbp_drone_base)) (Variables|/Script/Engine.PhysicsThrusterComponent|GetThrustStrength (Variables|/Script/DroneStabilization.DroneBase|GetPhysicsThrusterFL _asbp_drone_base)) (Variables|/Script/Engine.PhysicsThrusterComponent|GetThrustStrength (Variables|/Script/DroneStabilization.DroneBase|GetPhysicsThrusterFR _asbp_drone_base))) (Variables|Default|GetEnginesMultiplier))))

(fn ChangeParameters
  (params (Charge :type Float%20%28double-precision%29))
  (bind _returnvalue (== Charge 0.0))
  (bind _color (Variables|Default|GetColor))
  (if _returnvalue
    (if (not (Variables|Default|GetDisabledAll))
      (Variables|Default|SetDisabledAll true)
      (bind _aswbp_charge (Utilities|Casting|CastToWBP_Charge (UserInterface|GetWidget (Variables|Default|GetWidget)) :!label _label))
      (Default|SetChargeNumber _aswbp_charge Charge)
      (if (> Charge 50)
        (Rendering|Material|SetVectorParameterValue _color "Param" "(R=0.075611,G=1.000000,B=0.000000,A=1.000000)" :!class /Script/Engine.MaterialInstanceDynamic)
        (bind _asbp_drone_base (Utilities|Casting|CastToBP_DroneBase (Components|GetOwner)))
        (Rendering|Material|SetScalarParameterValue (Variables|/Game/Drone/Blueprints/BP_DroneBase.BP_DroneBase_C|GetMaterial _asbp_drone_base) "Hue Shift Percentage" 0.33 :!class /Script/Engine.MaterialInstanceDynamic)
        (Rendering|Material|SetScalarParameterValue (Variables|/Game/Drone/Blueprints/BP_DroneBase.BP_DroneBase_C|GetMaterial _asbp_drone_base) "Emissive Intesity" 2e+02 :!class /Script/Engine.MaterialInstanceDynamic)
        (elif (> Charge 20)
          (Rendering|Material|SetVectorParameterValue _color "Param" "(R=0.900000,G=1.000000,B=0.000000,A=1.000000)" :!class /Script/Engine.MaterialInstanceDynamic)
          (bind _asbp_drone_base_2 (Utilities|Casting|CastToBP_DroneBase (Components|GetOwner)))
          (Rendering|Material|SetScalarParameterValue (Variables|/Game/Drone/Blueprints/BP_DroneBase.BP_DroneBase_C|GetMaterial _asbp_drone_base_2) "Hue Shift Percentage" 0.2 :!class /Script/Engine.MaterialInstanceDynamic)
          (Rendering|Material|SetScalarParameterValue (Variables|/Game/Drone/Blueprints/BP_DroneBase.BP_DroneBase_C|GetMaterial _asbp_drone_base_2) "Emissive Intesity" 2e+02 :!class /Script/Engine.MaterialInstanceDynamic)
          (else
            (Rendering|Material|SetVectorParameterValue _color "Param" "(R=1.000000,G=0.000000,B=0.000000,A=1.000000)" :!class /Script/Engine.MaterialInstanceDynamic)
            (bind _asbp_drone_base_3 (Utilities|Casting|CastToBP_DroneBase (Components|GetOwner)))
            (Rendering|Material|SetScalarParameterValue (Variables|/Game/Drone/Blueprints/BP_DroneBase.BP_DroneBase_C|GetMaterial _asbp_drone_base_3) "Hue Shift Percentage" 0.0 :!class /Script/Engine.MaterialInstanceDynamic)
            (Rendering|Material|SetScalarParameterValue (Variables|/Game/Drone/Blueprints/BP_DroneBase.BP_DroneBase_C|GetMaterial _asbp_drone_base_3) "Emissive Intesity" 2e+02 :!class /Script/Engine.MaterialInstanceDynamic)
            (if _returnvalue
              (Rendering|Material|SetVectorParameterValue _color "Param" "(R=0.000000,G=0.000000,B=0.000000,A=1.000000)" :!class /Script/Engine.MaterialInstanceDynamic)
              (Rendering|Material|SetScalarParameterValue (Variables|/Game/Drone/Blueprints/BP_DroneBase.BP_DroneBase_C|GetMaterial _asbp_drone_base_3) "Emissive Intesity" 0.0 :!class /Script/Engine.MaterialInstanceDynamic)
              (Default|PoweronServer _asbp_drone_base_3 true false)
              (Default|ActivateShieldServer _asbp_drone_base_3 false))))))
    (else
      (Utilities|FlowControl|Sequence
        (:then_0
          (Variables|Default|SetDisabledAll false))
        (:then_1
          (goto _label))))))

(fn ShieldUsage
  (bind _asbp_drone_base (Utilities|Casting|CastToBP_DroneBase (Components|GetOwner)))
  (if (Variables|/Game/Drone/Shield/BP_ShieldBase.BP_ShieldBase_C|GetbIsActive (Default|GetShield _asbp_drone_base))
    (return (Variables|Default|GetShieldMultiplier))))