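; Drone stabilization component that corrects its owning BP_DroneBase each tick while engines and stabilization are enabled.
; A neural mode runs machine-learning corrections on vertical, rotation, front-back and left-right axes through ApplyML, replacing the vertical and rotation PIDs.
; Front-back and left-right PIDs with velocity smoothing parameters, then ApplyPID, run in both modes.
; Curves scale every PID multiplier except vertical, and all corrections are given min/max limits.
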(event EventBeginPlay)

(event EventTick
  (params (DeltaSeconds :type Float%20%28single-precision%29))
  (bind _asbp_drone_base (Utilities|Casting|CastToBP_DroneBase (Components|GetOwner)))
  (if (and (Variables|/Script/DroneStabilization.DroneBase|GetbIsEnginesActivated _asbp_drone_base) (Variables|/Script/DroneStabilization.DroneBase|GetbIsStabilizationEnabled _asbp_drone_base))
    (if (Variables|/Script/DroneStabilization.DroneBase|GetbIsNeuralStabilization _asbp_drone_base)
      ;[1 1 1] Mashine Learning
      (Class|StabilizationComponentBase|AllAxisML _asbp_drone_base "Vertical" (Variables|VerticalDelta|GetVerticalFL) (Variables|VerticalDelta|GetVerticalFR) (Variables|VerticalDelta|GetVerticalBL) (Variables|VerticalDelta|GetVerticalBR) (Variables|Parameter|GetVerticalParameter) -1.9e+02 3.9e+02)
      (Class|StabilizationComponentBase|AllAxisML _asbp_drone_base "Rotation" (Variables|RotationDelta|GetRotationFL) (Variables|RotationDelta|GetRotationFR) (Variables|RotationDelta|GetRotationBL) (Variables|RotationDelta|GetRotationBR) (Variables|Parameter|GetRotationParameter) -1.9e+02 3.9e+02)
      (Class|StabilizationComponentBase|AllAxisML _asbp_drone_base "FrontBack" (Variables|FrontBackDelta|GetFrontBackFL) (Variables|FrontBackDelta|GetFrontBackFR) (Variables|FrontBackDelta|GetFrontBackBL) (Variables|FrontBackDelta|GetFrontBackBR) (Variables|Parameter|GetFrontBackParameter) -1.9e+02 3.9e+02)
      (Class|StabilizationComponentBase|AllAxisML _asbp_drone_base "LeftRight" (Variables|LeftRightDelta|GetLeftRightFL) (Variables|LeftRightDelta|GetLeftRightFR) (Variables|LeftRightDelta|GetLeftRightBL) (Variables|LeftRightDelta|GetLeftRightBR) (Variables|Parameter|GetLeftRightParameter) -1.9e+02 3.9e+02)
      (Class|StabilizationComponentBase|ApplyML _asbp_drone_base 5.0 2e+02 -1.9e+02 3.9e+02)
      (else
        ;[1 1 1] PID
        (Class|StabilizationComponentBase|VerticalPID _asbp_drone_base DeltaSeconds (Utilities|Struct|MakeStabilizationParametersPID 0.7 0.005 0.05 0.0) 1.0 -2e+02 4e+02)
        (Class|StabilizationComponentBase|RotationPID _asbp_drone_base DeltaSeconds (Utilities|Struct|MakeStabilizationParametersPID 0.3 0.005 0.03 0.0) (Class|StabilizationComponentBase|GetMultiplierbyCurve "/Game/Drone/Blueprints/Curves/RotationMagnitude.RotationMagnitude" _asbp_drone_base 0.0001 1e+01) -2e+02 4e+02)))
    (Class|StabilizationComponentBase|FrontBacklPID _asbp_drone_base DeltaSeconds (Utilities|Struct|MakeStabilizationParametersPID 0.6 0.005 0.1 0.0) (Class|StabilizationComponentBase|GetMultiplierbyCurve "/Game/Drone/Blueprints/Curves/FrontBackMagnitude.FrontBackMagnitude" _asbp_drone_base 0.0001 1e+01) 1e+01 -2e+02 4e+02 (Utilities|Struct|MakeSmoothParametersPID -35.0 15.0 25.0 15.0 1e+01))
    (Class|StabilizationComponentBase|LeftRightPID _asbp_drone_base DeltaSeconds (Utilities|Struct|MakeStabilizationParametersPID 0.6 0.005 0.1 0.0) (Class|StabilizationComponentBase|GetMultiplierbyCurve "/Game/Drone/Blueprints/Curves/LeftRightMagnitude.LeftRightMagnitude" _asbp_drone_base 0.0001 1e+01) 1e+01 -2e+02 4e+02 (Utilities|Struct|MakeSmoothParametersPID 35.0 15.0 25.0 15.0 1e+01))
    (Class|StabilizationComponentBase|ApplyPID _asbp_drone_base 5.0 -2e+02 4e+02)))