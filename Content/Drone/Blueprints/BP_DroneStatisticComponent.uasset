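; Drone component that logs flight telemetry from its owning BP_DroneBase while logging is enabled.
; The IA_StartLog input action toggles logging on and off.
; Each Tick prints a semicolon-separated line of body-relative velocity, roll, pitch and the drone mesh's world Z angular velocity in degrees.
; Output goes only through Print String, with no file writing.
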(event Input|EnhancedActionEvents|EnhancedInputActionIA_StartLog
  (params (ActionValue :type Boolean) (ElapsedSeconds :type Float%20%28double-precision%29) (TriggeredSeconds :type Float%20%28double-precision%29) (InputAction :type Input%20Action%20Object%20Reference :default "/Game/Drone/Input/IA_StartLog.IA_StartLog"))
  (:Started
    (if (Variables|Default|GetbIsLogging)
      (Variables|Default|SetbIsLogging false)
      (else
        (Variables|Default|SetbIsLogging true)))))

(event EventBeginPlay)

(event EventTick
  (params (DeltaSeconds :type Float%20%28single-precision%29))
  (if (Variables|Default|GetbIsLogging)
    (bind _asbp_drone_base (Utilities|Casting|CastToBP_DroneBase (Components|GetOwner)))
    (Development|PrintString (Utilities|String|Append (Utilities|String|ToString(Float) (.x (Math|Vector|UnrotateVector (Transformation|GetVelocity _asbp_drone_base) (Transformation|GetActorRotation _asbp_drone_base)))) ";" (Utilities|String|ToString(Float) (.y (Math|Vector|UnrotateVector (Transformation|GetVelocity _asbp_drone_base) (Transformation|GetActorRotation _asbp_drone_base)))) ";" (Utilities|String|ToString(Float) (.z (Math|Vector|UnrotateVector (Transformation|GetVelocity _asbp_drone_base) (Transformation|GetActorRotation _asbp_drone_base)))) ";" (Utilities|String|ToString(Float) (.roll (Transformation|GetActorRotation _asbp_drone_base))) ";" (Utilities|String|ToString(Float) (.pitch (Transformation|GetActorRotation _asbp_drone_base))) ";" (Utilities|String|ToString(Float) (.z (Physics|GetPhysicsAngularVelocityinDegrees (Variables|/Script/DroneStabilization.DroneBase|GetDroneMesh _asbp_drone_base) "None")))))))