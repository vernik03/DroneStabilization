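; Player controller for a loading level that runs the possessed BP_DroneBase through a scripted sequence without player input.
; On BeginPlay it powers on the drone, then after a delay starts aiming and activates the weapon.
; Tick counts frames to apply a short negative power trigger, then fires every frame.
; It also has a pause menu toggle, while loading-widget and hardware-benchmark nodes are left disconnected.
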(event Custom|Loading%20begin%20play
  (bind _asbp_drone_base (Utilities|Casting|CastToBP_DroneBase (Pawn|GetControlledPawn)))
  (Default|PoweronServer _asbp_drone_base false false)
  (Utilities|FlowControl|Delay 4.0)
  (Default|AimingStartedServer _asbp_drone_base)
  (Variables|/Game/Drone/Weapons/BP_WeaponBase.BP_WeaponBase_C|SetbIsActivated (Default|GetWeapon _asbp_drone_base) true))

(event Custom|Loading%20Drone
  (bind _frame (Variables|Default|GetFrame))
  (bind _asbp_drone_base (Utilities|Casting|CastToBP_DroneBase (Pawn|GetControlledPawn)))
  (Math|Integer|IncrementInt _frame
    (:%20%20
      (if (not (< _frame 300))
        (if (< _frame 330)
          (Default|PowerAllTriggeredServer _asbp_drone_base -0.1)
          (else
            (Default|ShootServer _asbp_drone_base)))))))

(event EventBeginPlay
  (Actor|Tick|SetActorTickEnabled false)
  (CallFunction|LoadingBeginPlay)
  (Utilities|FlowControl|Delay 0.2)
  (Actor|Tick|SetActorTickEnabled true))

(event EventTick
  (params (DeltaSeconds :type Float%20%28single-precision%29))
  (CallFunction|LoadingDrone))

(fn ConstructionScript)

(fn PauseMenuChangeVisibility
  (bind _asbp_drone_hud (Utilities|Casting|CastToBP_DroneHUD (HUD|GetHUD)))
  (if (Widget|IsVisible (Variables|/Game/Drone/HUD/Blueprints/BP_DroneHUD.BP_DroneHUD_C|GetPause _asbp_drone_hud))
    (Default|HideSelf (Variables|/Game/Drone/HUD/Blueprints/BP_DroneHUD.BP_DroneHUD_C|GetPause _asbp_drone_hud))
    (Input|SetInputModeGameOnly self false)
    (Variables|Default|SetbShowMouseCursor false)
    (else
      (Default|ShowSelf (Variables|/Game/Drone/HUD/Blueprints/BP_DroneHUD.BP_DroneHUD_C|GetPause _asbp_drone_hud))
      (Input|SetInputModeGameandUI self (Variables|/Game/Drone/HUD/Blueprints/BP_DroneHUD.BP_DroneHUD_C|GetPause _asbp_drone_hud) "DoNotLock" false false)
      (Variables|Default|SetbShowMouseCursor true))))