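; BP_DroneHUD is the drone's HUD, showing the main widget and a separate aim reticle on screen.
; On BeginPlay it creates WBP_MainWidget and WBP_Aim for the owning player and adds both to the viewport.
; Each tick it reads AimScreenPosition from BP_PlayerController and eases the reticle toward it with VInterpTo, storing the smoothed position for the next frame.
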(event EventBeginPlay
  (bind _returnvalue (Game|Player|GetOwningPlayerController))
  (bind _returnvalue_2 (UserInterface|CreateWidget "/Game/Drone/HUD/Blueprints/WBP_MainWidget.WBP_MainWidget_C" _returnvalue))
  (UserInterface|Viewport|AddtoViewport _returnvalue_2 0)
  (Variables|Default|SetMainWidget _returnvalue_2)
  (bind _returnvalue_3 (UserInterface|CreateWidget "/Game/Drone/HUD/Blueprints/WBP_Aim.WBP_Aim_C" _returnvalue))
  (UserInterface|Viewport|AddtoViewport _returnvalue_3 0)
  (Variables|Default|SetAim _returnvalue_3))

(event Collision|EventActorBeginOverlap
  (params (OtherActor :type Actor%20Object%20Reference)))

(event EventTick
  (params (DeltaSeconds :type Float%20%28single-precision%29))
  (bind _asbp_player_controller (Utilities|Casting|CastToBP_PlayerController (Game|Player|GetOwningPlayerController)))
  (Class|UserWidget|SetPositioninViewport (Variables|Default|GetAim) (Math|Vector2D|MakeVector2D (.x (Math|Interpolation|VInterpTo (Math|Vector|MakeVector (.x (Variables|Default|GetAim%20Screen%20Position)) (.y (Variables|Default|GetAim%20Screen%20Position)) 0.0) (Math|Vector|MakeVector (.x (Variables|/Game/Drone/Blueprints/BP_PlayerController.BP_PlayerController_C|GetAimScreenPosition _asbp_player_controller)) (.y (Variables|/Game/Drone/Blueprints/BP_PlayerController.BP_PlayerController_C|GetAimScreenPosition _asbp_player_controller)) 0.0) DeltaSeconds 1e+01)) (.y (Math|Interpolation|VInterpTo (Math|Vector|MakeVector (.x (Variables|Default|GetAim%20Screen%20Position)) (.y (Variables|Default|GetAim%20Screen%20Position)) 0.0) (Math|Vector|MakeVector (.x (Variables|/Game/Drone/Blueprints/BP_PlayerController.BP_PlayerController_C|GetAimScreenPosition _asbp_player_controller)) (.y (Variables|/Game/Drone/Blueprints/BP_PlayerController.BP_PlayerController_C|GetAimScreenPosition _asbp_player_controller)) 0.0) DeltaSeconds 1e+01))) true)
  (Variables|Default|SetAim%20Screen%20Position (Math|Vector2D|MakeVector2D (.x (Math|Interpolation|VInterpTo (Math|Vector|MakeVector (.x (Variables|Default|GetAim%20Screen%20Position)) (.y (Variables|Default|GetAim%20Screen%20Position)) 0.0) (Math|Vector|MakeVector (.x (Variables|/Game/Drone/Blueprints/BP_PlayerController.BP_PlayerController_C|GetAimScreenPosition _asbp_player_controller)) (.y (Variables|/Game/Drone/Blueprints/BP_PlayerController.BP_PlayerController_C|GetAimScreenPosition _asbp_player_controller)) 0.0) DeltaSeconds 1e+01)) (.y (Math|Interpolation|VInterpTo (Math|Vector|MakeVector (.x (Variables|Default|GetAim%20Screen%20Position)) (.y (Variables|Default|GetAim%20Screen%20Position)) 0.0) (Math|Vector|MakeVector (.x (Variables|/Game/Drone/Blueprints/BP_PlayerController.BP_PlayerController_C|GetAimScreenPosition _asbp_player_controller)) (.y (Variables|/Game/Drone/Blueprints/BP_PlayerController.BP_PlayerController_C|GetAimScreenPosition _asbp_player_controller)) 0.0) DeltaSeconds 1e+01)))))

(fn ConstructionScript)