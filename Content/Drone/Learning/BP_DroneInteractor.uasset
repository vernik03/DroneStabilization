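; Learning Agents interactor that defines what the ML policy sees and controls on the BP_Drone_PAwn drone.
; Observes location, velocity, skeletal-mesh angular velocity and rotation, each relative to the drone's own transform, so location and rotation carry no world pose.
; Outputs four float actions, one per rotor corner, scaled and written to the StabilizationComponent's MLDelta values rather than applying forces itself.
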(fn SpecifyAgentObservation
  (params (InObservationSchema :type Learning%20Agents%20Observation%20Schema%20Object%20Reference))
  (return (Class|LearningAgentsObservations|SpecifyStructObservation InObservationSchema (Utilities|Map|MakeMap "Location" (Class|LearningAgentsObservations|SpecifyLocationObservation InObservationSchema) "Velocity" (Class|LearningAgentsObservations|SpecifyVelocityObservation InObservationSchema) "AngularVelocity" (Class|LearningAgentsObservations|SpecifyVelocityObservation InObservationSchema "AngularVelocityObservation") "RotationObservation" (Class|LearningAgentsObservations|SpecifyRotationObservation InObservationSchema)))))

(fn GatherAgentObservation
  (params (InObservationObject :type Learning%20Agents%20Observation%20Object%20Object%20Reference) (AgentId :type Integer))
  (LocalVariables|SetObsActor (Class|LearningAgentsManagerListener|GetAgent AgentId "/Game/Drone/BP_Drone_PAwn.BP_Drone_PAwn_C"))
  (return (Class|LearningAgentsObservations|MakeStructObservation InObservationObject (Utilities|Map|MakeMap "Location" (Class|LearningAgentsObservations|MakeLocationObservation InObservationObject (Transformation|GetActorLocation (LocalVariables|GetObsActor)) (Transformation|GetActorTransform (LocalVariables|GetObsActor)) 1e+04 "LocationObservation" false 0) "Velocity" (Class|LearningAgentsObservations|MakeVelocityObservation InObservationObject (Transformation|GetVelocity (LocalVariables|GetObsActor)) (Transformation|GetActorTransform (LocalVariables|GetObsActor)) 2e+02 "VelocityObservation" true 0) "AngularVelocity" (Class|LearningAgentsObservations|MakeVelocityObservation InObservationObject (Physics|GetPhysicsAngularVelocityinDegrees (Variables|/Game/Drone/BP_Drone_PAwn.BP_Drone_PAwn_C|GetSkeletalMesh (LocalVariables|GetObsActor)) "None") (Transformation|GetActorTransform (LocalVariables|GetObsActor)) 5e+01 "VelocityObservation" true 0) "RotationObservation" (Class|LearningAgentsObservations|MakeRotationObservation InObservationObject (Transformation|GetActorRotation (LocalVariables|GetObsActor)) (.rotation (Transformation|GetActorTransform (LocalVariables|GetObsActor))) "RotationObservation" false 0)))))

(fn SpecifyAgentAction
  (params (InActionSchema :type Learning%20Agents%20Action%20Schema%20Object%20Reference))
  (return (Class|LearningAgentsActions|SpecifyStructAction InActionSchema (Utilities|Map|MakeMap "PowerFL" (Class|LearningAgentsActions|SpecifyFloatAction InActionSchema "PowerFL") "PowerFR" (Class|LearningAgentsActions|SpecifyFloatAction InActionSchema "PowerFR") "PowerBL" (Class|LearningAgentsActions|SpecifyFloatAction InActionSchema "PowerBL") "PowerBR" (Class|LearningAgentsActions|SpecifyFloatAction InActionSchema "PowerBR")))))

(fn PerformAgentAction
  (params (InActionObject :type Learning%20Agents%20Action%20Object%20Object%20Reference) (InActionObjectElement :type Learning%20Agents%20Action%20Object%20Element%20Structure%20%28by%20ref%29) (AgentId :type Integer))
  (bind _scale (LocalVariables|GetScale))
  (LocalVariables|SetActActor (Class|LearningAgentsManagerListener|GetAgent AgentId "/Game/Drone/BP_Drone_PAwn.BP_Drone_PAwn_C"))
  (bind _outelements (Class|LearningAgentsActions|GetStructAction InActionObject InActionObjectElement))
  (Utilities|FlowControl|Sequence
    (:then_0
      (bind _outvalue (Class|LearningAgentsActions|GetFloatAction InActionObject (.Value (Utilities|Map|Find _outelements "PowerFL")) _scale "PowerFL" true 0))
      (Variables|/Game/Drone/StabilizationComponent.StabilizationComponent_C|SetMLDeltaFL (Variables|/Game/Drone/BP_Drone_PAwn.BP_Drone_PAwn_C|GetStabilizationComponent (LocalVariables|GetActActor)) _outvalue))
    (:then_1
      (bind _outvalue_2 (Class|LearningAgentsActions|GetFloatAction InActionObject (.Value (Utilities|Map|Find _outelements "PowerFR")) _scale "PowerFR" true 0))
      (Variables|/Game/Drone/StabilizationComponent.StabilizationComponent_C|SetMLDeltaFR (Variables|/Game/Drone/BP_Drone_PAwn.BP_Drone_PAwn_C|GetStabilizationComponent (LocalVariables|GetActActor)) _outvalue_2))
    (:then_2
      (bind _outvalue_3 (Class|LearningAgentsActions|GetFloatAction InActionObject (.Value (Utilities|Map|Find _outelements "PowerBL")) _scale "PowerBL" true 0))
      (Variables|/Game/Drone/StabilizationComponent.StabilizationComponent_C|SetMLDeltaBL (Variables|/Game/Drone/BP_Drone_PAwn.BP_Drone_PAwn_C|GetStabilizationComponent (LocalVariables|GetActActor)) _outvalue_3))
    (:then_3
      (bind _outvalue_4 (Class|LearningAgentsActions|GetFloatAction InActionObject (.Value (Utilities|Map|Find _outelements "PowerBR")) _scale "PowerBR" true 0))
      (Variables|/Game/Drone/StabilizationComponent.StabilizationComponent_C|SetMLDeltaBR (Variables|/Game/Drone/BP_Drone_PAwn.BP_Drone_PAwn_C|GetStabilizationComponent (LocalVariables|GetActActor)) _outvalue_4))))