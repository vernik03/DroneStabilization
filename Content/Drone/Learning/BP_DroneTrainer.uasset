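; Learning Agents trainer that teaches drone pawns to hover steadily and level.
; Rewards near-zero velocity, yaw spin and roll/pitch, with penalties past a threshold for each, by feeding these values into location-based reward helpers as vectors.
; Episodes complete when any of the three exceeds a wider limit.
; Episode reset returns the drone to its start position.
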(fn GatherAgentReward
  (params (AgentId :type Integer))
  (LocalVariables|SetRewardActor (Class|LearningAgentsManagerListener|GetAgent AgentId "/Game/Drone/BP_Drone_PAwn.BP_Drone_PAwn_C"))
  (return (+ (Class|LearningAgentsRewards|MakeRewardfromLocationSimilarity (Transformation|GetVelocity (LocalVariables|GetRewardActor)) "0, 0, 0" 1e+02 1e+01 "LocationSimilarityReward" false 0) (Class|LearningAgentsRewards|MakeRewardonLocationDifferenceAboveThreshold (Transformation|GetVelocity (LocalVariables|GetRewardActor)) "0, 0, 0" 7e+02 -5.0 "LocationDifferenceAboveThresholdReward" true 0) (Class|LearningAgentsRewards|MakeRewardfromLocationSimilarity (Math|Vector|MakeVector 0.0 0.0 (.z (Physics|GetPhysicsAngularVelocityinDegrees (Variables|/Game/Drone/BP_Drone_PAwn.BP_Drone_PAwn_C|GetSkeletalMesh (LocalVariables|GetRewardActor)) "None"))) "0, 0, 0" 3e+01 1e+01 "LocationSimilarityReward" false 0) (Class|LearningAgentsRewards|MakeRewardonLocationDifferenceAboveThreshold (Math|Vector|MakeVector 0.0 0.0 (.z (Physics|GetPhysicsAngularVelocityinDegrees (Variables|/Game/Drone/BP_Drone_PAwn.BP_Drone_PAwn_C|GetSkeletalMesh (LocalVariables|GetRewardActor)) "None"))) "0, 0, 0" 1.5e+02 -5.0 "LocationDifferenceAboveThresholdReward" true 0) (Class|LearningAgentsRewards|MakeRewardfromLocationSimilarity (Math|Vector|MakeVector (.roll (Transformation|GetActorRotation (LocalVariables|GetRewardActor))) (.pitch (Transformation|GetActorRotation (LocalVariables|GetRewardActor))) 0.0) "0, 0, 0" 5.0 1e+01 "LocationSimilarityReward" false 0) (Class|LearningAgentsRewards|MakeRewardonLocationDifferenceAboveThreshold (Math|Vector|MakeVector (.roll (Transformation|GetActorRotation (LocalVariables|GetRewardActor))) (.pitch (Transformation|GetActorRotation (LocalVariables|GetRewardActor))) 0.0) "0, 0, 0" 45.0 -5.0 "LocationDifferenceAboveThresholdReward" true 0))))

(fn GatherAgentCompletion
  (params (AgentId :type Integer))
  (bind _returnvalue (Class|LearningAgentsManagerListener|GetAgent AgentId "/Game/Drone/BP_Drone_PAwn.BP_Drone_PAwn_C"))
  (bind _returnvalue_2 (Transformation|GetActorRotation _returnvalue))
  (return (Class|LearningAgentsCompletions|Completionor (Class|LearningAgentsCompletions|MakeCompletiononLocationDifferenceAboveThreshold (Transformation|GetVelocity _returnvalue) "0, 0, 0" 2e+03 "Termination" "LocationDifferenceAboveThresholdCompletion" false 0) (Class|LearningAgentsCompletions|MakeCompletiononLocationDifferenceAboveThreshold (Math|Vector|MakeVector 0.0 0.0 (.z (Physics|GetPhysicsAngularVelocityinDegrees (Variables|/Game/Drone/BP_Drone_PAwn.BP_Drone_PAwn_C|GetSkeletalMesh _returnvalue) "None"))) "0, 0, 0" 2e+02 "Termination" "LocationDifferenceAboveThresholdCompletion" false 0) (Class|LearningAgentsCompletions|MakeCompletiononLocationDifferenceAboveThreshold (Math|Vector|MakeVector (.roll _returnvalue_2) (.pitch _returnvalue_2) 0.0) "0, 0, 0" 8e+01 "Termination" "LocationDifferenceAboveThresholdCompletion" false 0))))

(fn ResetAgentEpisode
  (params (AgentId :type Integer))
  (Default|ResettoStartPosition (Class|LearningAgentsManagerListener|GetAgent AgentId "/Game/Drone/BP_Drone_PAwn.BP_Drone_PAwn_C")))