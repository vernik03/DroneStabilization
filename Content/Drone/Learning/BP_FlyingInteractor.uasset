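; Learning Agents interactor that defines what BP_Drone_PAwn agents observe and control when learning to fly.
; Observations cover goal position relative to the drone, planar orientation on three planes, velocity and distance to goal.
; The goal is captured once at setup from the location of the first BP_Drone_PAwn found, not a separate target.
; Four float actions write each agent's FR, FL, BR and BL rotor tick power.
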(event EventSetupObservations
  (Utilities|FlowControl|Sequence
    (:then_0
      (bind _returnvalue (Class|PositionObservation|AddPositionObservation 0 "PositionObservation" 1e+03))
      (Variables|Default|SetPositionObservation _returnvalue)
      (bind _returnvalue_2 (Class|PlanarDirectionObservation|AddPlanarDirectionObservation 0 "PlanarDirectionObservationXY" 1.0 "1.000000,0.000000,0.000000" "0.000000,1.000000,0.000000"))
      (Variables|Default|SetPlanarDirectionObservationXY _returnvalue_2)
      (bind _returnvalue_3 (Class|PlanarDirectionObservation|AddPlanarDirectionObservation 0 "PlanarDirectionObservationXZ" 1.0 "1.000000,0.000000,0.000000" "0.000000,0.000000,1.000000"))
      (Variables|Default|SetPlanarDirectionObservationXZ _returnvalue_3)
      (bind _returnvalue_4 (Class|PlanarDirectionObservation|AddPlanarDirectionObservation 0 "PlanarDirectionObservationYZ" 1.0 "0.000000,1.000000,0.000000" "0.000000,0.000000,1.000000"))
      (Variables|Default|SetPlanarDirectionObservationYZ _returnvalue_4))
    (:then_1
      (bind _returnvalue_5 (Class|VelocityObservation|AddVelocityObservation 0 "VelocityObservation" 2e+02))
      (Variables|Default|SetVelocityObservation _returnvalue_5))
    (:then_2
      (bind _returnvalue_6 (Actor|GetActorOfClass "/Game/Drone/BP_Drone_PAwn.BP_Drone_PAwn_C"))
      (Variables|Default|SetGoalLocation (Transformation|GetActorLocation _returnvalue_6)))
    (:then_3
      ;[0.06447 1 0.9861] Modified:
      (bind _returnvalue_7 (Class|FloatObservation|AddFloatObservation 0 "Distance" 1e+03))
      (Variables|Default|SetDistanceObs _returnvalue_7))))

(event EventSetObservations
  (params (AgentIds :type Array%20of%20Integers))
  (for _array_element AgentIds
    (Utilities|FlowControl|Sequence
      (:then_0
        ;[0.5922 1 0.1531] ✅
        (Class|PositionObservation|SetPositionObservation (Variables|Default|GetPositionObservation) _array_element (Variables|Default|GetGoalLocation) (.location (Transformation|GetActorTransform (Class|LearningAgentsManagerComponent|GetAgent _array_element "/Game/Drone/BP_Drone_PAwn.BP_Drone_PAwn_C"))) (.rotation (Transformation|GetActorTransform (Class|LearningAgentsManagerComponent|GetAgent _array_element "/Game/Drone/BP_Drone_PAwn.BP_Drone_PAwn_C")))))
      (:then_1
        (Class|PlanarDirectionObservation|SetPlanarDirectionObservation (Variables|Default|GetPlanarDirectionObservationXY) _array_element (Math|Vector|MakeVector 0.0 0.0 0.0) (Transformation|GetActorRotation (Class|LearningAgentsManagerComponent|GetAgent _array_element "/Game/Drone/BP_Drone_PAwn.BP_Drone_PAwn_C")))
        (Class|PlanarDirectionObservation|SetPlanarDirectionObservation (Variables|Default|GetPlanarDirectionObservationXZ) _array_element (Math|Vector|MakeVector 0.0 0.0 0.0) (Transformation|GetActorRotation (Class|LearningAgentsManagerComponent|GetAgent _array_element "/Game/Drone/BP_Drone_PAwn.BP_Drone_PAwn_C")))
        (Class|PlanarDirectionObservation|SetPlanarDirectionObservation (Variables|Default|GetPlanarDirectionObservationYZ) _array_element (Math|Vector|MakeVector 0.0 0.0 0.0) (Transformation|GetActorRotation (Class|LearningAgentsManagerComponent|GetAgent _array_element "/Game/Drone/BP_Drone_PAwn.BP_Drone_PAwn_C"))))
      (:then_3
        (Class|VelocityObservation|SetVelocityObservation (Variables|Default|GetVelocityObservation) _array_element (Transformation|GetVelocity (Class|LearningAgentsManagerComponent|GetAgent _array_element "/Game/Drone/BP_Drone_PAwn.BP_Drone_PAwn_C")) (Transformation|GetActorRotation (Class|LearningAgentsManagerComponent|GetAgent _array_element "/Game/Drone/BP_Drone_PAwn.BP_Drone_PAwn_C"))))
      (:then_4
        (Class|FloatObservation|SetFloatObservation (Variables|Default|GetDistanceObs) _array_element (Math|Vector|Distance(Vector) (Transformation|GetActorLocation (Class|LearningAgentsManagerComponent|GetAgent _array_element "/Game/Drone/BP_Drone_PAwn.BP_Drone_PAwn_C")) (Variables|Default|GetGoalLocation)))))))

(event EventSetupActions
  (Utilities|FlowControl|Sequence
    (:then_0
      (bind _returnvalue (Class|FloatAction|AddFloatAction 0 "FR Power Action" 2.0))
      (Variables|Default|SetFR%20Power _returnvalue))
    (:then_1
      (bind _returnvalue_2 (Class|FloatAction|AddFloatAction 0 "FL Power Action" 2.0))
      (Variables|Default|SetFL%20Power _returnvalue_2))
    (:then_2
      (bind _returnvalue_3 (Class|FloatAction|AddFloatAction 0 "BR Power Action" 2.0))
      (Variables|Default|SetBR%20Power _returnvalue_3))
    (:then_3
      (bind _returnvalue_4 (Class|FloatAction|AddFloatAction 0 "BL Power Action" 2.0))
      (Variables|Default|SetBL%20Power _returnvalue_4))))

(event EventGetActions
  (params (AgentIds :type Array%20of%20Integers))
  (for _array_element AgentIds
    (Utilities|FlowControl|Sequence
      (:then_0
        (bind _returnvalue (Class|FloatAction|GetFloatAction (Variables|Default|GetFL%20Power) _array_element))
        (bind _output_get (Variables|/Game/Drone/BP_Drone_PAwn.BP_Drone_PAwn_C|SetFL_TickPower (Class|LearningAgentsManagerComponent|GetAgent _array_element "/Game/Drone/BP_Drone_PAwn.BP_Drone_PAwn_C") _returnvalue)))
      (:then_1
        (bind _returnvalue_2 (Class|FloatAction|GetFloatAction (Variables|Default|GetFR%20Power) _array_element))
        (bind _output_get_2 (Variables|/Game/Drone/BP_Drone_PAwn.BP_Drone_PAwn_C|SetFR_TickPower (Class|LearningAgentsManagerComponent|GetAgent _array_element "/Game/Drone/BP_Drone_PAwn.BP_Drone_PAwn_C") _returnvalue_2)))
      (:then_2
        (bind _returnvalue_3 (Class|FloatAction|GetFloatAction (Variables|Default|GetBR%20Power) _array_element))
        (bind _output_get_3 (Variables|/Game/Drone/BP_Drone_PAwn.BP_Drone_PAwn_C|SetBR_TickPower (Class|LearningAgentsManagerComponent|GetAgent _array_element "/Game/Drone/BP_Drone_PAwn.BP_Drone_PAwn_C") _returnvalue_3)))
      (:then_3
        (bind _returnvalue_4 (Class|FloatAction|GetFloatAction (Variables|Default|GetBL%20Power) _array_element))
        (bind _output_get_4 (Variables|/Game/Drone/BP_Drone_PAwn.BP_Drone_PAwn_C|SetBL_TickPower (Class|LearningAgentsManagerComponent|GetAgent _array_element "/Game/Drone/BP_Drone_PAwn.BP_Drone_PAwn_C") _returnvalue_4))))))