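; Learning Agents trainer that teaches drones to hold position at the spot where a BP_Drone_PAwn stood at BeginPlay.
; Rewards combine per-plane distance penalties with a tiered bonus from three nested boxes around the target, drawn as debug boxes.
; Straying too far in any plane triggers completion, and episode resets return drones to the target.
; Collision, speed and angular-velocity terms are unwired; the bound hit handler only casts.
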(event Custom|HitEventDispatcher_Event
  (params (HitActor :type Actor%20Object%20Reference) (SelfActor :type Actor%20Object%20Reference))
  (bind _asbp_drone_pawn (Utilities|Casting|CastToBP_Drone_PAwn SelfActor)))

(event EventSetupRewards
  (Utilities|FlowControl|Sequence
    (:then_0
      (bind _returnvalue (Class|PlanarPositionDifferencePenalty|AddPlanarPositionDifferencePenalty 0 "Off_XY_Penalty" 1.0 1e+02 8e+02 "1.000000,0.000000,0.000000" "0.000000,1.000000,0.000000"))
      (Variables|Default|SetOff_XY_Penalty _returnvalue))
    (:then_1
      (bind _returnvalue_2 (Class|PlanarPositionDifferencePenalty|AddPlanarPositionDifferencePenalty 0 "Off_XZ_Penalty" 1.0 1e+02 8e+02 "1.000000,0.000000,0.000000" "0.000000,0.000000,1.000000"))
      (Variables|Default|SetOff_XZ_Penalty _returnvalue_2))
    (:then_2
      (bind _returnvalue_3 (Class|PlanarPositionDifferencePenalty|AddPlanarPositionDifferencePenalty 0 "Off_YZ_Penalty" 1.0 1e+02 8e+02 "0.000000,1.000000,0.000000" "0.000000,0.000000,1.000000"))
      (Variables|Default|SetOff_YZ_Penalty _returnvalue_3))
    (:then_6
      (bind _returnvalue_4 (Class|FloatReward|AddFloatReward 0 "PositionReward" 2.0))
      (Variables|Default|SetPositionReward _returnvalue_4))))

(event EventSetRewards
  (params (AgentIds :type Array%20of%20Integers))
  (bind _targetposition (Variables|Default|GetTargetPosition))
  (bind _positionreward (Variables|Default|GetPositionReward))
  (bind _targetposition_2 (Variables|Default|GetTargetPosition))
  (for _array_element AgentIds
    (Utilities|FlowControl|Sequence
      (:then_0
        (Utilities|FlowControl|Sequence
          (:then_0
            (Class|PlanarPositionDifferencePenalty|SetPlanarPositionDifferencePenalty (Variables|Default|GetOff_XY_Penalty) _array_element (Transformation|GetActorLocation (Class|LearningAgentsManagerComponent|GetAgent _array_element "/Game/Drone/BP_Drone_PAwn.BP_Drone_PAwn_C")) _targetposition_2))
          (:then_1
            (Class|PlanarPositionDifferencePenalty|SetPlanarPositionDifferencePenalty (Variables|Default|GetOff_XZ_Penalty) _array_element (Transformation|GetActorLocation (Class|LearningAgentsManagerComponent|GetAgent _array_element "/Game/Drone/BP_Drone_PAwn.BP_Drone_PAwn_C")) _targetposition_2))
          (:then_2
            (Class|PlanarPositionDifferencePenalty|SetPlanarPositionDifferencePenalty (Variables|Default|GetOff_YZ_Penalty) _array_element (Transformation|GetActorLocation (Class|LearningAgentsManagerComponent|GetAgent _array_element "/Game/Drone/BP_Drone_PAwn.BP_Drone_PAwn_C")) _targetposition_2))))
      (:then_2
        (if (Math|Geometry|IsPointinBox (Transformation|GetActorLocation (Class|LearningAgentsManagerComponent|GetAgent _array_element "/Game/Drone/BP_Drone_PAwn.BP_Drone_PAwn_C")) _targetposition (Math|Conversions|ToVector(Float) (Variables|Default|GetBox1)))
          (Class|FloatReward|SetFloatReward _positionreward _array_element 1e+01)
          (Rendering|Debug|DrawDebugBox _targetposition (Math|Conversions|ToVector(Float) (Variables|Default|GetBox1)) "(R=0.044869,G=1.000000,B=0.000000,A=1.000000)" "0, 0, 0" 1.0 5.0)
          (elif (Math|Geometry|IsPointinBox (Transformation|GetActorLocation (Class|LearningAgentsManagerComponent|GetAgent _array_element "/Game/Drone/BP_Drone_PAwn.BP_Drone_PAwn_C")) _targetposition (Math|Conversions|ToVector(Float) (Variables|Default|GetBox2)))
            (Class|FloatReward|SetFloatReward _positionreward _array_element 5.0)
            (Rendering|Debug|DrawDebugBox _targetposition (Math|Conversions|ToVector(Float) (Variables|Default|GetBox2)) "(R=1.000000,G=0.460151,B=0.000000,A=1.000000)" "0, 0, 0" 1.0 5.0)
            (elif (Math|Geometry|IsPointinBox (Transformation|GetActorLocation (Class|LearningAgentsManagerComponent|GetAgent _array_element "/Game/Drone/BP_Drone_PAwn.BP_Drone_PAwn_C")) _targetposition (Math|Conversions|ToVector(Float) (Variables|Default|GetBox3)))
              (Class|FloatReward|SetFloatReward _positionreward _array_element 2.0)
              (Rendering|Debug|DrawDebugBox _targetposition (Math|Conversions|ToVector(Float) (Variables|Default|GetBox3)) "(R=1.000000,G=0.028557,B=0.000000,A=1.000000)" "0, 0, 0" 1.0 5.0)
              (else
                (Class|FloatReward|SetFloatReward _positionreward _array_element 0.0))))))
      (:then_3
        (EventDispatchers|AssignHitEventDispatcher (Class|LearningAgentsManagerComponent|GetAgent _array_element "/Game/Drone/BP_Drone_PAwn.BP_Drone_PAwn_C") (delegate Custom|HitEventDispatcher_Event))))))

(event EventSetupCompletions
  (Utilities|FlowControl|Sequence
    (:then_0
      (bind _returnvalue (Class|PlanarPositionDifferenceCompletion|AddPlanarPositionDifferenceCompletion 0 "Off_XY_Termination" 1.5e+03 "Termination" "1.000000,0.000000,0.000000" "0.000000,1.000000,0.000000"))
      (Variables|Default|SetOff_XY_Termination _returnvalue))
    (:then_1
      (bind _returnvalue_2 (Class|PlanarPositionDifferenceCompletion|AddPlanarPositionDifferenceCompletion 0 "Off_XZ_Termination" 1.5e+03 "Termination" "1.000000,0.000000,0.000000" "0.000000,0.000000,1.000000"))
      (Variables|Default|SetOff_XZ_Termination _returnvalue_2))
    (:then_2
      (bind _returnvalue_3 (Class|PlanarPositionDifferenceCompletion|AddPlanarPositionDifferenceCompletion 0 "Off_YZ_Termination" 1.5e+03 "Termination" "0.000000,1.000000,0.000000" "0.000000,0.000000,1.000000"))
      (Variables|Default|SetOff_YZ_Termination _returnvalue_3))))

(event EventResetEpisodes
  (params (AgentIds :type Array%20of%20Integers))
  (for _array_element AgentIds
    (Default|ResettoPosition (Class|LearningAgentsManagerComponent|GetAgent _array_element "/Game/Drone/BP_Drone_PAwn.BP_Drone_PAwn_C") (Variables|Default|GetTargetPosition))))

(event EventBeginPlay
  (bind _returnvalue (Actor|GetActorOfClass "/Game/Drone/BP_Drone_PAwn.BP_Drone_PAwn_C"))
  (Variables|Default|SetTargetPosition (Transformation|GetActorLocation _returnvalue)))

(event EventSetCompletions
  (params (AgentIds :type Array%20of%20Integers))
  (for _array_element AgentIds
    (Utilities|FlowControl|Sequence
      (:then_0
        (Class|PlanarPositionDifferenceCompletion|SetPlanarPositionDifferenceCompletion (Variables|Default|GetOff_XY_Termination) _array_element (Variables|Default|GetTargetPosition) (Transformation|GetActorLocation (Class|LearningAgentsManagerComponent|GetAgent _array_element "/Game/Drone/BP_Drone_PAwn.BP_Drone_PAwn_C"))))
      (:then_1
        (Class|PlanarPositionDifferenceCompletion|SetPlanarPositionDifferenceCompletion (Variables|Default|GetOff_YZ_Termination) _array_element (Variables|Default|GetTargetPosition) (Transformation|GetActorLocation (Class|LearningAgentsManagerComponent|GetAgent _array_element "/Game/Drone/BP_Drone_PAwn.BP_Drone_PAwn_C"))))
      (:then_2
        (Class|PlanarPositionDifferenceCompletion|SetPlanarPositionDifferenceCompletion (Variables|Default|GetOff_XZ_Termination) _array_element (Variables|Default|GetTargetPosition) (Transformation|GetActorLocation (Class|LearningAgentsManagerComponent|GetAgent _array_element "/Game/Drone/BP_Drone_PAwn.BP_Drone_PAwn_C")))))))