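; Learning Agents interactor that defines what a BP_DroneBase agent observes and how its policy drives the drone.
; Observations are a struct of location, linear velocity, angular velocity from the drone mesh physics and rotation, each taken relative to the drone's own transform.
; Actions are four floats (FB, LR, V, H), scaled, clamped and written to the matching parameters on the drone's stabilization component.
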(fn SpecifyAgentObservation
  (params (InObservationSchema :type Learning%20Agents%20Observation%20Schema%20Object%20Reference))
  (return (Class|LearningAgentsObservations|SpecifyStructObservation InObservationSchema (Utilities|Map|MakeMap "LocationObservation" (Class|LearningAgentsObservations|SpecifyLocationObservation InObservationSchema) "VelocityObservation" (Class|LearningAgentsObservations|SpecifyVelocityObservation InObservationSchema) "AngularVelocityObservation" (Class|LearningAgentsObservations|SpecifyVelocityObservation InObservationSchema "AngularVelocityObservation") "RotationObservation" (Class|LearningAgentsObservations|SpecifyRotationObservation InObservationSchema)))))

(fn GatherAgentObservation
  (params (InObservationObject :type Learning%20Agents%20Observation%20Object%20Object%20Reference) (AgentId :type Integer))
  (LocalVariables|SetObsActor (Class|LearningAgentsManagerListener|GetAgent AgentId "/Game/Drone/BP_DroneBase.BP_DroneBase_C"))
  (return (Class|LearningAgentsObservations|MakeStructObservation InObservationObject (Utilities|Map|MakeMap "LocationObservation" (Class|LearningAgentsObservations|MakeLocationObservation InObservationObject (Transformation|GetActorLocation (LocalVariables|GetObsActor)) (Transformation|GetActorTransform (LocalVariables|GetObsActor)) 1e+04 "LocationObservation" false 0) "VelocityObservation" (Class|LearningAgentsObservations|MakeVelocityObservation InObservationObject (Transformation|GetVelocity (LocalVariables|GetObsActor)) (Transformation|GetActorTransform (LocalVariables|GetObsActor)) 2e+02 "VelocityObservation" true 0) "AngularVelocityObservation" (Class|LearningAgentsObservations|MakeVelocityObservation InObservationObject (Physics|GetPhysicsAngularVelocityinDegrees (Variables|/Script/DroneStabilization.DroneBase|GetDroneMesh (LocalVariables|GetObsActor)) "None") (Transformation|GetActorTransform (LocalVariables|GetObsActor)) 5e+01 "AngularVelocityObservation" true 0) "RotationObservation" (Class|LearningAgentsObservations|MakeRotationObservation InObservationObject (Transformation|GetActorRotation (LocalVariables|GetObsActor)) (.rotation (Transformation|GetActorTransform (LocalVariables|GetObsActor))) "RotationObservation" false 0)))))

(fn SpecifyAgentAction
  (params (InActionSchema :type Learning%20Agents%20Action%20Schema%20Object%20Reference))
  (return (Class|LearningAgentsActions|SpecifyStructAction InActionSchema (Utilities|Map|MakeMap "ParameterFB" (Class|LearningAgentsActions|SpecifyFloatAction InActionSchema "ParameterFB") "ParameterLR" (Class|LearningAgentsActions|SpecifyFloatAction InActionSchema "ParameterLR") "ParameterV" (Class|LearningAgentsActions|SpecifyFloatAction InActionSchema "ParameterV") "ParameterH" (Class|LearningAgentsActions|SpecifyFloatAction InActionSchema "ParameterH")))))

(fn PerformAgentAction
  (params (InActionObject :type Learning%20Agents%20Action%20Object%20Object%20Reference) (InActionObjectElement :type Learning%20Agents%20Action%20Object%20Element%20Structure%20%28by%20ref%29) (AgentId :type Integer))
  (bind _scale (LocalVariables|GetScale))
  (bind _max (LocalVariables|GetMax))
  (bind _min (LocalVariables|GetMin))
  (bind _max_2 (LocalVariables|GetMax))
  (bind _min_2 (LocalVariables|GetMin))
  (LocalVariables|SetActActor (Class|LearningAgentsManagerListener|GetAgent AgentId "/Game/Drone/BP_DroneBase.BP_DroneBase_C"))
  (bind _outelements (Class|LearningAgentsActions|GetStructAction InActionObject InActionObjectElement))
  (Utilities|FlowControl|Sequence
    (:then_0
      (bind _outvalue (Class|LearningAgentsActions|GetFloatAction InActionObject (.Value (Utilities|Map|Find _outelements "ParameterFB")) _scale "ParameterFB" true 0))
      (Variables|/Game/Drone/DroneStabilizationComponent.DroneStabilizationComponent_C|SetFB_Parameter (Variables|/Game/Drone/BP_DroneBase.BP_DroneBase_C|GetDroneStabilizationComponent (LocalVariables|GetActActor)) (Math|Float|Clamp(Float) _outvalue _min _max_2)))
    (:then_1
      (bind _outvalue_2 (Class|LearningAgentsActions|GetFloatAction InActionObject (.Value (Utilities|Map|Find _outelements "ParameterLR")) _scale "ParameterLR" true 0))
      (Variables|/Game/Drone/DroneStabilizationComponent.DroneStabilizationComponent_C|SetLR_Parameter (Variables|/Game/Drone/BP_DroneBase.BP_DroneBase_C|GetDroneStabilizationComponent (LocalVariables|GetActActor)) (Math|Float|Clamp(Float) _outvalue_2 _min _max_2)))
    (:then_2
      (bind _outvalue_3 (Class|LearningAgentsActions|GetFloatAction InActionObject (.Value (Utilities|Map|Find _outelements "ParameterV")) _scale "ParameterV" true 0))
      (Variables|/Game/Drone/DroneStabilizationComponent.DroneStabilizationComponent_C|SetV_Parameter (Variables|/Game/Drone/BP_DroneBase.BP_DroneBase_C|GetDroneStabilizationComponent (LocalVariables|GetActActor)) (Math|Float|Clamp(Float) _outvalue_3 _min_2 _max)))
    (:then_3
      (bind _outvalue_4 (Class|LearningAgentsActions|GetFloatAction InActionObject (.Value (Utilities|Map|Find _outelements "ParameterH")) _scale "ParameterH" true 0))
      (Variables|/Game/Drone/DroneStabilizationComponent.DroneStabilizationComponent_C|SetH_Parameter (Variables|/Game/Drone/BP_DroneBase.BP_DroneBase_C|GetDroneStabilizationComponent (LocalVariables|GetActActor)) (Math|Float|Clamp(Float) _outvalue_4 _min_2 _max)))))