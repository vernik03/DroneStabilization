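; Learning Agents trainer that teaches BP_DroneBase agents to hold a stable, level hover.
; Rewards favor near-zero body-space velocity, yaw rate and roll/pitch, with stepped penalties when these exceed set thresholds.
; An episode completes on excessive speed, spin or tilt, and reset is delegated to the drone's ResetDrone.
; Location-similarity and distance helpers are reused for angles and rates by packing them into vector components.
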(fn GatherAgentReward
  (params (AgentId :type Integer))
  (LocalVariables|SetRewardActor (Class|LearningAgentsManagerListener|GetAgent AgentId "/Game/Drone/BP_DroneBase.BP_DroneBase_C"))
  (return (+ (Class|LearningAgentsRewards|MakeRewardfromLocationSimilarity (Math|Vector|UnrotateVector (Transformation|GetVelocity (LocalVariables|GetRewardActor)) (Transformation|GetActorRotation (LocalVariables|GetRewardActor))) "0, 0, 0" 1e+02 5.0 "LocationSimilarityReward" false 0) (Class|LearningAgentsRewards|MakeRewardonLocationDifferenceAboveThreshold (Math|Vector|UnrotateVector (Transformation|GetVelocity (LocalVariables|GetRewardActor)) (Transformation|GetActorRotation (LocalVariables|GetRewardActor))) "0, 0, 0" 7e+02 -5.0 "LocationDifferenceAboveThresholdReward" true 0) (Class|LearningAgentsRewards|MakeRewardfromLocationSimilarity (Math|Vector|MakeVector 0.0 0.0 (.z (Physics|GetPhysicsAngularVelocityinDegrees (Variables|/Script/DroneStabilization.DroneBase|GetDroneMesh (LocalVariables|GetRewardActor)) "None"))) "0, 0, 0" 3e+01 5.0 "LocationSimilarityReward" false 0) (Class|LearningAgentsRewards|MakeRewardonLocationDifferenceAboveThreshold (Math|Vector|MakeVector 0.0 0.0 (.z (Physics|GetPhysicsAngularVelocityinDegrees (Variables|/Script/DroneStabilization.DroneBase|GetDroneMesh (LocalVariables|GetRewardActor)) "None"))) "0, 0, 0" 1.5e+02 -5.0 "LocationDifferenceAboveThresholdReward" true 0) (Class|LearningAgentsRewards|MakeRewardfromLocationSimilarity (Math|Vector|MakeVector (.roll (Transformation|GetActorRotation (LocalVariables|GetRewardActor))) (.pitch (Transformation|GetActorRotation (LocalVariables|GetRewardActor))) 0.0) "0, 0, 0" 5.0 5.0 "LocationSimilarityReward" false 0) (Class|LearningAgentsRewards|MakeRewardonLocationDifferenceAboveThreshold (Math|Vector|MakeVector (.roll (Transformation|GetActorRotation (LocalVariables|GetRewardActor))) (.pitch (Transformation|GetActorRotation (LocalVariables|GetRewardActor))) 0.0) "0, 0, 0" 4e+01 -5.0 "LocationDifferenceAboveThresholdReward" true 0) (Class|LearningAgentsRewards|MakeRewardonLocationDifferenceAboveThreshold (Math|Vector|MakeVector (.roll (Transformation|GetActorRotation (LocalVariables|GetRewardActor))) (.pitch (Transformation|GetActorRotation (LocalVariables|GetRewardActor))) 0.0) "0, 0, 0" 1e+02 -5e+01 "LocationDifferenceAboveThresholdReward" true 0))))

(fn GatherAgentCompletion
  (params (AgentId :type Integer))
  (bind _returnvalue (Class|LearningAgentsManagerListener|GetAgent AgentId "/Game/Drone/BP_DroneBase.BP_DroneBase_C"))
  (bind _returnvalue_2 (Transformation|GetActorRotation _returnvalue))
  (return (Class|LearningAgentsCompletions|Completionor (Class|LearningAgentsCompletions|MakeCompletiononLocationDifferenceAboveThreshold (Transformation|GetVelocity _returnvalue) "0, 0, 0" 3e+03 "Termination" "LocationDifferenceAboveThresholdCompletion" false 0) (Class|LearningAgentsCompletions|MakeCompletiononLocationDifferenceAboveThreshold (Math|Vector|MakeVector 0.0 0.0 (.z (Physics|GetPhysicsAngularVelocityinDegrees (Variables|/Script/DroneStabilization.DroneBase|GetDroneMesh _returnvalue) "None"))) "0, 0, 0" 3e+02 "Termination" "LocationDifferenceAboveThresholdCompletion" false 0) (Class|LearningAgentsCompletions|MakeCompletiononLocationDifferenceAboveThreshold (Math|Vector|MakeVector (.roll _returnvalue_2) (.pitch _returnvalue_2) 0.0) "0, 0, 0" 75.0 "Termination" "LocationDifferenceAboveThresholdCompletion" false 0))))

(fn ResetAgentEpisode
  (params (AgentId :type Integer))
  (Class|DroneBase|ResetDrone (Class|LearningAgentsManagerListener|GetAgent AgentId "/Game/Drone/BP_DroneBase.BP_DroneBase_C")))