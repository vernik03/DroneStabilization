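; Learning Agents trainer for the drone's horizontal rotation, rewarding it for keeping yaw spin near zero.
; It feeds the mesh's Z angular velocity into location-based reward helpers, combining a near-zero similarity reward with a penalty for fast spin.
; The same value triggers episode completion past a higher threshold, and episode reset returns the drone pawn to its start position.
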(fn GatherAgentReward
  (params (AgentId :type Integer))
  (LocalVariables|SetRewardActor (Class|LearningAgentsManagerListener|GetAgent AgentId "/Game/Drone/BP_Drone_PAwn.BP_Drone_PAwn_C"))
  (return (+ (Class|LearningAgentsRewards|MakeRewardfromLocationSimilarity (Math|Vector|MakeVector 0.0 0.0 (.z (Physics|GetPhysicsAngularVelocityinDegrees (Variables|/Game/Drone/BP_Drone_PAwn.BP_Drone_PAwn_C|GetSkeletalMesh (LocalVariables|GetRewardActor)) "None"))) "0, 0, 0" 2e+01 1e+01 "LocationSimilarityReward" false 0) (Class|LearningAgentsRewards|MakeRewardonLocationDifferenceAboveThreshold (Math|Vector|MakeVector 0.0 0.0 (.z (Physics|GetPhysicsAngularVelocityinDegrees (Variables|/Game/Drone/BP_Drone_PAwn.BP_Drone_PAwn_C|GetSkeletalMesh (LocalVariables|GetRewardActor)) "None"))) "0, 0, 0" 8e+01 -5.0 "LocationDifferenceAboveThresholdReward" true 0))))

(fn GatherAgentCompletion
  (params (AgentId :type Integer))
  (return (Class|LearningAgentsCompletions|MakeCompletiononLocationDifferenceAboveThreshold (Math|Vector|MakeVector 0.0 0.0 (.z (Physics|GetPhysicsAngularVelocityinDegrees (Variables|/Game/Drone/BP_Drone_PAwn.BP_Drone_PAwn_C|GetSkeletalMesh (Class|LearningAgentsManagerListener|GetAgent AgentId "/Game/Drone/BP_Drone_PAwn.BP_Drone_PAwn_C")) "None"))) "0, 0, 0" 1.2e+02 "Termination" "LocationDifferenceAboveThresholdCompletion" false 0)))

(fn ResetAgentEpisode
  (params (AgentId :type Integer))
  (Default|ResettoStartPosition (Class|LearningAgentsManagerListener|GetAgent AgentId "/Game/Drone/BP_Drone_PAwn.BP_Drone_PAwn_C")))