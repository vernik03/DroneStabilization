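; Learning Agents interactor for the drone's left-right learning task, defining what the agent observes and controls on BP_DroneBase.
; Observes location, velocity, mesh angular velocity and rotation, each expressed relative to the drone's own transform, so location and rotation are self-referenced.
; Outputs two scaled float actions, PowerL and PowerR, written to the stabilization component's LeftRight values, each driving the front and back rotor on its side.
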(fn SpecifyAgentObservation
  (params (InObservationSchema :type Learning%20Agents%20Observation%20Schema%20Object%20Reference))
  (return (Class|LearningAgentsObservations|SpecifyStructObservation InObservationSchema (Utilities|Map|MakeMap "LocationObservation" (Class|LearningAgentsObservations|SpecifyLocationObservation InObservationSchema) "VelocityObservation" (Class|LearningAgentsObservations|SpecifyVelocityObservation InObservationSchema) "AngularVelocityObservation" (Class|LearningAgentsObservations|SpecifyVelocityObservation InObservationSchema "AngularVelocityObservation") "RotationObservation" (Class|LearningAgentsObservations|SpecifyRotationObservation InObservationSchema)))))

(fn GatherAgentObservation
  (params (InObservationObject :type Learning%20Agents%20Observation%20Object%20Object%20Reference) (AgentId :type Integer))
  (LocalVariables|SetObsActor (Class|LearningAgentsManagerListener|GetAgent AgentId "/Game/Drone/BP_DroneBase.BP_DroneBase_C"))
  (return (Class|LearningAgentsObservations|MakeStructObservation InObservationObject (Utilities|Map|MakeMap "LocationObservation" (Class|LearningAgentsObservations|MakeLocationObservation InObservationObject (Transformation|GetActorLocation (LocalVariables|GetObsActor)) (Transformation|GetActorTransform (LocalVariables|GetObsActor)) 1e+04 "LocationObservation" false 0) "VelocityObservation" (Class|LearningAgentsObservations|MakeVelocityObservation InObservationObject (Transformation|GetVelocity (LocalVariables|GetObsActor)) (Transformation|GetActorTransform (LocalVariables|GetObsActor)) 2e+02 "VelocityObservation" true 0) "AngularVelocityObservation" (Class|LearningAgentsObservations|MakeVelocityObservation InObservationObject (Physics|GetPhysicsAngularVelocityinDegrees (Variables|/Script/DroneStabilization.DroneBase|GetDroneMesh (LocalVariables|GetObsActor)) "None") (Transformation|GetActorTransform (LocalVariables|GetObsActor)) 5e+01 "AngularVelocityObservation" true 0) "RotationObservation" (Class|LearningAgentsObservations|MakeRotationObservation InObservationObject (Transformation|GetActorRotation (LocalVariables|GetObsActor)) (.rotation (Transformation|GetActorTransform (LocalVariables|GetObsActor))) "RotationObservation" false 0)))))

(fn SpecifyAgentAction
  (params (InActionSchema :type Learning%20Agents%20Action%20Schema%20Object%20Reference))
  (return (Class|LearningAgentsActions|SpecifyStructAction InActionSchema (Utilities|Map|MakeMap "PowerL" (Class|LearningAgentsActions|SpecifyFloatAction InActionSchema "PowerL") "PowerR" (Class|LearningAgentsActions|SpecifyFloatAction InActionSchema "PowerR")))))

(fn PerformAgentAction
  (params (InActionObject :type Learning%20Agents%20Action%20Object%20Object%20Reference) (InActionObjectElement :type Learning%20Agents%20Action%20Object%20Element%20Structure%20%28by%20ref%29) (AgentId :type Integer))
  (bind _scale (LocalVariables|GetScale))
  (LocalVariables|SetActActor (Class|LearningAgentsManagerListener|GetAgent AgentId "/Game/Drone/BP_DroneBase.BP_DroneBase_C"))
  (bind _outelements (Class|LearningAgentsActions|GetStructAction InActionObject InActionObjectElement))
  (Utilities|FlowControl|Sequence
    (:then_0
      (bind _outvalue (Class|LearningAgentsActions|GetFloatAction InActionObject (.Value (Utilities|Map|Find _outelements "PowerL")) _scale "PowerL" true 0))
      (Utilities|FlowControl|Sequence
        (:then_0
          (Variables|/Game/Drone/DroneStabilizationComponent.DroneStabilizationComponent_C|SetLeftRightFL (Variables|/Game/Drone/BP_DroneBase.BP_DroneBase_C|GetDroneStabilizationComponent (LocalVariables|GetActActor)) _outvalue))
        (:then_1
          (Variables|/Game/Drone/DroneStabilizationComponent.DroneStabilizationComponent_C|SetLeftRightBL (Variables|/Game/Drone/BP_DroneBase.BP_DroneBase_C|GetDroneStabilizationComponent (LocalVariables|GetActActor)) _outvalue))))
    (:then_1
      (bind _outvalue_2 (Class|LearningAgentsActions|GetFloatAction InActionObject (.Value (Utilities|Map|Find _outelements "PowerR")) _scale "PowerR" true 0))
      (Utilities|FlowControl|Sequence
        (:then_0
          (Variables|/Game/Drone/DroneStabilizationComponent.DroneStabilizationComponent_C|SetLeftRightFR (Variables|/Game/Drone/BP_DroneBase.BP_DroneBase_C|GetDroneStabilizationComponent (LocalVariables|GetActActor)) _outvalue_2))
        (:then_1
          (Variables|/Game/Drone/DroneStabilizationComponent.DroneStabilizationComponent_C|SetLeftRightBR (Variables|/Game/Drone/BP_DroneBase.BP_DroneBase_C|GetDroneStabilizationComponent (LocalVariables|GetActActor)) _outvalue_2))))))