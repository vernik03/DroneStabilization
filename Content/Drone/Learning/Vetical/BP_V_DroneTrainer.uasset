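; Learning Agents trainer for the drone's vertical control, rewarding each BP_DroneBase agent for keeping vertical velocity near zero.
; Reward repurposes location helpers on Z velocity, combining a similarity bonus with a penalty for exceeding a speed threshold.
; An episode completes when vertical speed passes a higher limit, and resetting calls the drone's own ResetDrone.
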(fn GatherAgentReward
  (params (AgentId :type Integer))
  (LocalVariables|SetRewardActor (Class|LearningAgentsManagerListener|GetAgent AgentId "/Game/Drone/BP_DroneBase.BP_DroneBase_C"))
  (return (+ (Class|LearningAgentsRewards|MakeRewardfromLocationSimilarity (Math|Vector|MakeVector 0.0 0.0 (.z (Transformation|GetVelocity (LocalVariables|GetRewardActor)))) "0, 0, 0" 1e+02 1e+01 "LocationSimilarityReward" false 0) (Class|LearningAgentsRewards|MakeRewardonLocationDifferenceAboveThreshold (Math|Vector|MakeVector 0.0 0.0 (.z (Transformation|GetVelocity (LocalVariables|GetRewardActor)))) "0, 0, 0" 7e+02 -5.0 "LocationDifferenceAboveThresholdReward" true 0) 0.0 0.0 0.0 0.0)))

(fn GatherAgentCompletion
  (params (AgentId :type Integer))
  (return (Class|LearningAgentsCompletions|MakeCompletiononLocationDifferenceAboveThreshold (Math|Vector|MakeVector 0.0 0.0 (.z (Transformation|GetVelocity (Class|LearningAgentsManagerListener|GetAgent AgentId "/Game/Drone/BP_DroneBase.BP_DroneBase_C")))) "0, 0, 0" 2e+03 "Termination" "LocationDifferenceAboveThresholdCompletion" false 0)))

(fn ResetAgentEpisode
  (params (AgentId :type Integer))
  (Class|DroneBase|ResetDrone (Class|LearningAgentsManagerListener|GetAgent AgentId "/Game/Drone/BP_DroneBase.BP_DroneBase_C")))