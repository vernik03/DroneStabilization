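; Spline-driven wall Blueprint that tiles a static mesh along a spline, built in the construction script with no active event logic.
; Segment length comes from MeshLength, or from the mesh's X bounds when zero, and only whole segments are placed.
; Each segment is a spline mesh component with tangents clamped to segment length.
; StaticMaterials is written onto the static mesh itself rather than as component overrides.
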(event EventBeginPlay)

(event Collision|EventActorBeginOverlap
  (params (OtherActor :type Actor%20Object%20Reference)))

(event EventTick
  (params (DeltaSeconds :type Float%20%28single-precision%29)))

(fn ConstructionScript
  (bind _spline (Variables|Default|GetSpline))
  (if (== (Variables|Default|GetMeshLength) 0.0)
    (bind _mesh (Variables|Default|GetMesh)
      (:then
        (Variables|Default|SetMeshLength (.x (- (.max (StaticMesh|GetBoundingBox _mesh)) (.min (StaticMesh|GetBoundingBox _mesh))))))
      (:else)))
  (if (> (Math|Float|Truncate (/ (Spline|GetSplineLength (Variables|Default|GetSpline)) (Variables|Default|GetMeshLength))) 0)
    (for _index (range 0 (- (Math|Float|Truncate (/ (Spline|GetSplineLength (Variables|Default|GetSpline)) (Variables|Default|GetMeshLength))) 1))
      (bind _returnvalue (AddComponent|AddSplineMeshComponent false))
      (SplineMesh|SetStartandEnd _returnvalue (Spline|GetLocationatDistanceAlongSpline _spline (* _index (Variables|Default|GetMeshLength)) "Local") (Math|Vector|ClampVectorSize (Spline|GetTangentatDistanceAlongSpline _spline (* _index (Variables|Default|GetMeshLength)) "Local") 1.0 (Variables|Default|GetMeshLength)) (Spline|GetLocationatDistanceAlongSpline _spline (* (+ _index 1) (Variables|Default|GetMeshLength)) "Local") (Math|Vector|ClampVectorSize (Spline|GetTangentatDistanceAlongSpline _spline (* (+ _index 1) (Variables|Default|GetMeshLength)) "Local") 1.0 (Variables|Default|GetMeshLength)) true :!class /Script/Engine.SplineMeshComponent)
      (Components|StaticMesh|SetStaticMesh _returnvalue (Variables|Default|GetMesh))
      (Transformation|AttachComponentToComponent _returnvalue (Variables|Default|GetSpline) "None" "KeepRelative" "KeepRelative" "KeepRelative" true)
      (Variables|/Script/Engine.StaticMesh|SetStaticMaterials (Variables|/Script/Engine.StaticMeshComponent|GetStaticMesh _returnvalue) (Variables|Default|GetStatic%20Materials)))))