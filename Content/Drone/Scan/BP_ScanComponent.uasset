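; Scan component for a DroneBase owner that fades a post-process scan effect in and out.
; StartScan and EndScan drive a state machine whose normalized time advances on Tick, with both fades using FadeInSpeed.
; That time sets the blend weight, optionally through a curve, on a lazily spawned BP_Scan_Actor carrying a dynamic material.
; MPC_Scan receives state, time and drone location; Inactive disables Tick and optionally destroys the actor.
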(event EventBeginPlay
  (bind _asdrone_base (Utilities|Casting|CastToDroneBase (Components|GetOwner))
    (:then
      (Variables|Default|SetPlayerController _asdrone_base)
      (CallFunction|UpdateScanState true "NewEnumerator3")
      (Rendering|Material|SetScalarParameterValue "/Game/Drone/Scan/MPC_Scan.MPC_Scan" "GridCellSize" (Variables|Default|GetGridCellSize) :!class /Script/Engine.KismetMaterialLibrary)
      (Rendering|Material|SetScalarParameterValue "/Game/Drone/Scan/MPC_Scan.MPC_Scan" "Range" (Variables|Default|GetRange) :!class /Script/Engine.KismetMaterialLibrary))
    (:CastFailed
      (CallFunction|UpdateScanState false "NewEnumerator4"))))

(event EventTick
  (params (DeltaSeconds :type Float%20%28single-precision%29))
  (bind _playercontroller (Variables|Default|GetPlayerController))
  (CallFunction|UpdateScanTime DeltaSeconds)
  (Development|PrintString (Utilities|String|ToString(Float) (Variables|Default|GetScanNormalizedTime)) true false "(R=0.000000,G=0.660000,B=1.000000,A=1.000000)" 0.0)
  (Development|PrintString (Utilities|String|EnumtoString (Variables|Default|GetScanState)) true false "(R=0.000000,G=0.660000,B=1.000000,A=1.000000)" 0.0)
  (switch Utilities|FlowControl|Switch|SwitchonEBP_Scan_State (CallFunction|GetScanState)
    (:NewEnumerator0
      _)
    (:NewEnumerator1
      _)
    (:NewEnumerator2
      _)
    (:NewEnumerator3
      _))
  (CallFunction|UpdateScanPPBlendWeight)
  (Utilities|IsValid _playercontroller
    (:Is%20Valid
      (Rendering|Material|SetVectorParameterValue "/Game/Drone/Scan/MPC_Scan.MPC_Scan" "Location" (Math|Conversions|ToLinearColor(Vector) (Transformation|GetActorLocation _playercontroller)) :!class /Script/Engine.KismetMaterialLibrary))))

(fn StartScan
  (Development|PrintString (Utilities|String|EnumtoString (Variables|Default|GetScanState)))
  (switch Utilities|FlowControl|Switch|SwitchonEBP_Scan_State (CallFunction|GetScanState)
    (:NewEnumerator2
      _)
    (:NewEnumerator3
      _))
  (CallFunction|UpdateScanState false "NewEnumerator0"))

(fn EndScan
  (switch Utilities|FlowControl|Switch|SwitchonEBP_Scan_State (CallFunction|GetScanState)
    (:NewEnumerator0
      _)
    (:NewEnumerator1
      _))
  (CallFunction|UpdateScanState false "NewEnumerator2"))

(fn GetScanState
  (return (Variables|Default|GetScanState)))

(fn UpdateScanState
  (params (Force :type Boolean) (State :type EBP_Scan_State%20Enum :default "NewEnumerator0"))
  (Development|PrintString "Change")
  (Development|PrintString (Utilities|String|EnumtoString (Variables|Default|GetScanState)))
  (Development|PrintString (Utilities|String|EnumtoString State))
  (if (or Force (Utilities|Enum|NotEqual(Enum) State (Variables|Default|GetScanState)))
    (Utilities|FlowControl|Sequence
      (:then_0
        (switch Utilities|FlowControl|Switch|SwitchonEBP_Scan_State (Variables|Default|GetScanState)
          (:NewEnumerator1
            (Rendering|Material|SetScalarParameterValue "/Game/Drone/Scan/MPC_Scan.MPC_Scan" "bActive" 0.0 :!class /Script/Engine.KismetMaterialLibrary))
          (:NewEnumerator3
            (Rendering|Material|SetScalarParameterValue "/Game/Drone/Scan/MPC_Scan.MPC_Scan" "bInactive" 0.0 :!class /Script/Engine.KismetMaterialLibrary)
            (Components|Tick|SetComponentTickEnabled true))))
      (:then_1
        (bind _output_get (Variables|Default|SetScanState State))
        (switch Utilities|FlowControl|Switch|SwitchonEBP_Scan_State _output_get
          (:NewEnumerator1
            (Rendering|Material|SetScalarParameterValue "/Game/Drone/Scan/MPC_Scan.MPC_Scan" "bActive" 1.0 :!class /Script/Engine.KismetMaterialLibrary)
            (CallFunction|UpdateScanPPBlendWeight))
          (:NewEnumerator3
            (Rendering|Material|SetScalarParameterValue "/Game/Drone/Scan/MPC_Scan.MPC_Scan" "bInactive" 1.0 :!class /Script/Engine.KismetMaterialLibrary)
            (CallFunction|UpdateScanPPBlendWeight)
            (Components|Tick|SetComponentTickEnabled false :!label _label)
            (CallFunction|DestroyPPActor))
          (:NewEnumerator4
            (goto _label))))
      (:then_2
        (return true)))
    (else
      (return false))))

(fn UpdateScanTime
  (params (DeltaTime :type Float%20%28double-precision%29))
  (Utilities|FlowControl|Sequence
    (:then_0
      (switch Utilities|FlowControl|Switch|SwitchonEBP_Scan_State (CallFunction|GetScanState)
        (:NewEnumerator0
          (bind _output_get (Variables|Default|SetScanNormalizedTime (+ (Variables|Default|GetScanNormalizedTime) (* DeltaTime (Variables|Default|GetFadeInSpeed)))))
          (if (>= _output_get 1.0)
            (CallFunction|UpdateScanState false "NewEnumerator1")))
        (:NewEnumerator2
          (bind _output_get_2 (Variables|Default|SetScanNormalizedTime (- (Variables|Default|GetScanNormalizedTime) (* DeltaTime (Variables|Default|GetFadeInSpeed)))))
          (if (<= _output_get_2 0.0)
            (CallFunction|UpdateScanState false "NewEnumerator3")))
        (:NewEnumerator4
          (return false)))
      (Rendering|Material|SetScalarParameterValue "/Game/Drone/Scan/MPC_Scan.MPC_Scan" "NormalizedTime" (Variables|Default|GetScanNormalizedTime) :!class /Script/Engine.KismetMaterialLibrary))
    (:then_1
      (return true))))

(fn GetScanPPActor
  (bind _ppmaterial (Variables|Default|GetPPMaterial))
  (Utilities|IsValid (Variables|Default|GetScanActor)
    (:Is%20Valid
      (return (Variables|Default|GetScanActor)))
    (:Is%20Not%20Valid
      (bind _returnvalue (Game|SpawnActorfromClass "/Game/Drone/Scan/BP_Scan_Actor.BP_Scan_Actor_C" (Math|Transform|MakeTransform "0, 0, 0") "Undefined" "MultiplyWithRoot" (Variables|Default|GetPlayerController) 0))
      (Variables|Default|SetScanActor _returnvalue)
      (Utilities|FlowControl|Sequence
        (:then_0
          (Utilities|IsValid (Variables|Default|GetPPMaterialDynamic)
            (:Is%20Valid
              _)
            (:Is%20Not%20Valid
              (Utilities|IsValid _ppmaterial
                (:Is%20Valid
                  (bind _returnvalue_2 (Rendering|Material|CreateDynamicMaterialInstance _ppmaterial "None" "None" :!class /Script/Engine.KismetMaterialLibrary))
                  (Variables|Default|SetPPMaterialDynamic _returnvalue_2)))))
          (Utilities|IsValid (Variables|/Game/Drone/Scan/BP_Scan_Actor.BP_Scan_Actor_C|GetPostProcess (Variables|Default|GetScanActor))
            (:Is%20Valid
              (Utilities|Struct|SetmembersinPostProcessSettings (Variables|/Script/Engine.PostProcessComponent|GetSettings (Variables|/Game/Drone/Scan/BP_Scan_Actor.BP_Scan_Actor_C|GetPostProcess (Variables|Default|GetScanActor))) (Utilities|Struct|MakeWeightedBlendables (Utilities|Array|MakeArray (Utilities|Struct|MakeWeightedBlendable 1.0 (Variables|Default|GetPPMaterialDynamic))))))))
        (:then_1
          (return (Variables|Default|GetScanActor)))))))

(fn DestroyPPActor
  (if (and (Variables|Default|GetbDestroyActor) (Utilities|IsValid (Variables|Default|GetScanActor)))
    (Actor|DestroyActor (Variables|Default|GetScanActor))
    (Variables|Default|SetScanActor 0)))

(fn UpdateScanPPBlendWeight
  (bind _blendcurve (Variables|Default|GetBlendCurve))
  (bind _scannormalizedtime (Variables|Default|GetScanNormalizedTime))
  (Utilities|IsValid _blendcurve
    (:Is%20Valid
      (LocalVariables|SetThisTime (Math|Curves|GetFloatValue _blendcurve _scannormalizedtime)))
    (:Is%20Not%20Valid
      (LocalVariables|SetThisTime _scannormalizedtime)))
  (bind _scanactor (CallFunction|GetScanPPActor))
  (Utilities|IsValid _scanactor
    (:Is%20Valid
      (Utilities|IsValid (Variables|/Game/Drone/Scan/BP_Scan_Actor.BP_Scan_Actor_C|GetPostProcess _scanactor)
        (:Is%20Valid
          (Variables|/Script/Engine.PostProcessComponent|SetBlendWeight (Variables|/Game/Drone/Scan/BP_Scan_Actor.BP_Scan_Actor_C|GetPostProcess _scanactor) (LocalVariables|GetThisTime)))))))