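; BP_Shooting_Small is a projectile emitter in the shield VFX folder that continuously spawns small ProjectileBP actors from BeginPlay onward.
; Each shot spawns at a random offset around the actor, scaled down and facing along its Arrow component.
; The NextArrow event re-triggers itself after a short random delay, forming an endless loop.
; The Z offset reuses the X-axis range, so there is no separate vertical range.
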(event Custom|NextArrow
  (bind _x_axis_min (Variables|Default|GetX%20axis%20Min))
  (bind _xaxis_max (Variables|Default|GetXaxis%20Max))
  (bind _returnvalue (Math|Random|RandomFloatinRange _x_axis_min _xaxis_max))
  (Game|SpawnActorfromClass (Variables|Default|GetProjectileBP) (Math|Transform|MakeTransform (+ (Transformation|GetActorLocation) (Math|Vector|MakeVector _returnvalue (Math|Random|RandomFloatinRange (Variables|Default|GetYaxis%20min) (Variables|Default|GetYaxis%20Max)) _returnvalue)) (.rotation (Transformation|GetWorldTransform (Variables|Default|GetArrow))) "0.100000,0.100000,0.100000") "Undefined" "SelectDefaultAtRuntime" 0 0)
  (Utilities|FlowControl|Delay (Math|Random|RandomFloatinRange 0.0 0.1))
  (CallFunction|NextArrow))

(event EventBeginPlay
  (bind _x_axis_min (Variables|Default|GetX%20axis%20Min))
  (bind _xaxis_max (Variables|Default|GetXaxis%20Max))
  (bind _returnvalue (Math|Random|RandomFloatinRange _x_axis_min _xaxis_max))
  (Utilities|FlowControl|Delay (Math|Random|RandomFloatinRange 0.0 0.1))
  (Game|SpawnActorfromClass (Variables|Default|GetProjectileBP) (Math|Transform|MakeTransform (+ (Transformation|GetActorLocation) (Math|Vector|MakeVector _returnvalue (Math|Random|RandomFloatinRange (Variables|Default|GetYaxis%20min) (Variables|Default|GetYaxis%20Max)) _returnvalue)) (.rotation (Transformation|GetWorldTransform (Variables|Default|GetArrow))) "0.100000,0.100000,0.100000") "Undefined" "SelectDefaultAtRuntime" 0 0)
  (Utilities|FlowControl|Delay (Math|Random|RandomFloatinRange 0.0 0.1))
  (CallFunction|NextArrow))

(fn ConstructionScript)