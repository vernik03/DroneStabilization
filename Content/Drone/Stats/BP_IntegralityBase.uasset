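; BP_IntegralityBase is a base health stat for the drone, tracking its integrity.
; Health starts at Max on BeginPlay, and the Damage and Repair functions lower or raise it, clamped between zero and Max.
; Damage calls the ZeroHealth dispatcher whenever the clamped result is zero, leaving the response to whatever is bound to it.
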(event EventBeginPlay
  (Variables|Default|SetHealth (Variables|Default|GetMax)))

(event EventTick
  (params (DeltaSeconds :type Float%20%28single-precision%29)))

(fn Damage
  (params (Damage :type Float%20%28double-precision%29))
  (bind _output_get (Variables|Default|SetHealth (Math|Float|Clamp(Float) (- (Variables|Default|GetHealth) Damage) 0.0 (Variables|Default|GetMax))))
  (if (== _output_get 0.0)
    (Default|CallZeroHealth)))

(fn Repair
  (params (Heal :type Float%20%28double-precision%29))
  (Variables|Default|SetHealth (Math|Float|Clamp(Float) (+ (Variables|Default|GetHealth) Heal) 0.0 (Variables|Default|GetMax))))