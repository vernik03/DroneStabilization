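; Base drone weapon that handles aiming, deployment along a spline via a reversible timeline, and firing with a reload cooldown.
; Shots fake travel time: a trace sets the delay from bullet speed, then a delayed re-trace applies curve-scaled damage to drones, cannons or shields.
; ShootBulletClient plays muzzle, tracer, impact, decal and sound effects on remote instances, timing impacts to bullet arrival.
; Remote Tick projects the barrel trace to the controller's screen aim point.
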(event Custom|DeactivateEvent
  (bind _weaponmesh (Variables|Default|GetWeaponMesh))
  (bind _spline (Variables|Default|GetSpline))
  (bind _relativerotation (Variables|/Script/Engine.SceneComponent|GetRelativeRotation _weaponmesh))
  (Variables|Default|SetbIsActivated false)
  (bind (_direction _movement _rotation) (Timeline|Timeline Reverse)
    (:Update
      (Utilities|FlowControl|Sequence
        (:then_0
          (Utilities|IsValid _spline
            (:Is%20Valid
              (Transformation|SetRelativeLocationAndRotation _weaponmesh (.location (Spline|GetTransformatDistanceAlongSpline (Variables|Default|GetSpline) (Math|Float|Lerp 0.0 (Spline|GetSplineLength _spline) _movement) "Local" false)) (Math|Rotator|MakeRotator (+ (* (.pitch (.rotation (Spline|GetTransformatDistanceAlongSpline (Variables|Default|GetSpline) (Math|Float|Lerp 0.0 (Spline|GetSplineLength _spline) _movement) "Local" false))) -1.0) 1.8e+02) (.pitch _relativerotation) (.yaw _relativerotation)) true false))))
        (:then_1
          (Variables|Default|SetAiming _rotation)
          (Variables|Default|SetRotation (Math|Float|Lerp (Variables|Default|GetRotation) 0.0 _movement)))))))

(event Custom|ActivateEvent
  (bind _weaponmesh (Variables|Default|GetWeaponMesh))
  (bind _spline (Variables|Default|GetSpline))
  (bind _relativerotation (Variables|/Script/Engine.SceneComponent|GetRelativeRotation _weaponmesh))
  (Variables|Default|SetbIsActivated true)
  (bind (_direction _movement _rotation) (Timeline|Timeline Play)
    (:Update
      (Utilities|FlowControl|Sequence
        (:then_0
          (Utilities|IsValid _spline
            (:Is%20Valid
              (Transformation|SetRelativeLocationAndRotation _weaponmesh (.location (Spline|GetTransformatDistanceAlongSpline (Variables|Default|GetSpline) (Math|Float|Lerp 0.0 (Spline|GetSplineLength _spline) _movement) "Local" false)) (Math|Rotator|MakeRotator (+ (* (.pitch (.rotation (Spline|GetTransformatDistanceAlongSpline (Variables|Default|GetSpline) (Math|Float|Lerp 0.0 (Spline|GetSplineLength _spline) _movement) "Local" false))) -1.0) 1.8e+02) (.pitch _relativerotation) (.yaw _relativerotation)) true false))))
        (:then_1
          (Variables|Default|SetAiming _rotation)
          (Variables|Default|SetRotation (Math|Float|Lerp (Variables|Default|GetRotation) 0.0 _movement)))))))

(event Custom|ShootBullet
  (bind _weaponmesh (Variables|Default|GetWeaponMesh))
  (bind _weaponmesh_2 (Variables|Default|GetWeaponMesh))
  (bind _weaponmesh_3 (Variables|Default|GetWeaponMesh))
  (bind _returnvalue (Transformation|GetSocketTransform _weaponmesh "ShootingPoint" "RTS_World"))
  (bind _returnvalue_2 (Transformation|GetSocketTransform _weaponmesh_2 "ShootingPoint" "RTS_World"))
  (bind _returnvalue_3 (Transformation|GetSocketLocation _weaponmesh_3 "BeginningOfBarrel"))
  (bind _returnvalue_4 (Math|Vector|GetUnitDirection(Vector) _returnvalue_3 (.location _returnvalue_2)))
  (bind _returnvalue_5 (* _returnvalue_4 5e+04))
  (bind _returnvalue_6 (+ _returnvalue_3 _returnvalue_5))
  (if (> (Variables|Default|GetReloadingTime) (Variables|Default|GetReloadingDuration))
    (Variables|Default|SetReloadingTime 0.0)
    (bind _asbp_drone_base (Utilities|Casting|CastToBP_DroneBase (Components|GetOwner)))
    (bind _outhit (Collision|LineTraceByChannel (.location _returnvalue_2) _returnvalue_6 "TraceTypeQuery3" false (Utilities|Array|MakeArray (Components|GetOwner) (Default|GetShield _asbp_drone_base)) "None"))
    (bind _output_get (Variables|Default|SetBulletTime (/ (.distance _outhit) (Variables|Default|GetBulletSpeed))))
    (CallFunction|Damage (.location _returnvalue_2) _returnvalue_6 _output_get)
    (bind _returnvalue_7 (Game|SpawnActorfromClass "/Game/Drone/Weapons/BulletByTrace.BulletByTrace_C" (Math|Transform|MakeTransform (.location _returnvalue) (Math|Rotator|MakeRotator (.roll (.rotation _returnvalue)) (.pitch (.rotation _returnvalue)) (.yaw (.rotation _returnvalue))) "1.000000,1.000000,1.000000") "Undefined" "MultiplyWithRoot" 0 0))
    (Actor|SetOwner _returnvalue_7 (Components|GetOwner))
    (Variables|/Game/Drone/Weapons/BulletByTrace.BulletByTrace_C|SetDuration _returnvalue_7 (Variables|Default|GetBulletTime))
    (CallFunction|ShootBulletClient (.location _outhit) (.normal _outhit) (Variables|/Script/PhysicsCore.PhysicalMaterial|GetSurfaceType (.physmat _outhit)))))

(event Custom|ShootBulletClient
  (params ([0] :type Vector) ([0]2 :type Vector) ([0]3 :type EPhysicalSurface%20Enum :default "SurfaceType_Default"))
  (Networking|SwitchHasAuthority
    (:Remote
      (Variables|Default|SetImpact%20Positions (Utilities|Array|MakeArray [0]))
      (Variables|Default|SetImpact%20Normals (Utilities|Array|MakeArray [0]2))
      (Variables|Default|SetImpactSurfaceTypes (Utilities|Array|MakeArray [0]3))
      (bind _output_get (Variables|Default|SetMuzzlePosition (Transformation|GetSocketLocation (Variables|Default|GetWeaponMesh) "ShootingPoint")))
      (Utilities|FlowControl|Sequence
        (:then_0
          ;[1 1 1] Spawn and activate Weapon Fire effects. We need seperate actors so as to not destroy the effects when switching to another weapon. The actors containing the effects gets destroyed when all systems are dead
          (Utilities|IsValid (Variables|Default|GetWeaponFire)
            (:Is%20Valid
              _)
            (:Is%20Not%20Valid
              (bind _returnvalue (Game|SpawnActorfromClass "/Game/Effects/Blueprints/B_WeaponFire.B_WeaponFire_C" (Math|Transform|MakeTransform "0, 0, 0") "Undefined" "OverrideRootScale" 0 (Variables|Default|GetWeaponMesh) false "/Game/Effects/Particles/Weapons/NS_WeaponFire_ShellEject.NS_WeaponFire_ShellEject" true "/Game/Effects/Particles/Weapons/NS_WeaponFire_MuzzleFlash_Rifle.NS_WeaponFire_MuzzleFlash_Rifle" true "/Game/Effects/Particles/Weapons/NS_WeaponFire_Tracer.NS_WeaponFire_Tracer" "/Game/Effects/Meshes/BulletShells/SM_rifleshell.SM_rifleshell" 0))
              (bind _output_get_2 (Variables|Default|SetWeaponFire _returnvalue))
              (Transformation|AttachComponentToComponent _output_get_2 (Variables|Default|GetWeaponMesh) "ShootingPoint" "KeepRelative" "KeepRelative" "KeepRelative" true)))
          (Variables|/Game/Effects/Blueprints/B_WeaponFire.B_WeaponFire_C|SetImpactPositions (Variables|Default|GetWeaponFire) (Variables|Default|GetImpact%20Positions))
          (Variables|/Game/Effects/Blueprints/B_WeaponFire.B_WeaponFire_C|SetImpactNormals (Variables|Default|GetWeaponFire) (Variables|Default|GetImpact%20Normals))
          (Variables|/Game/Effects/Blueprints/B_WeaponFire.B_WeaponFire_C|SetImpactSurfaceTypes (Variables|Default|GetWeaponFire) (Variables|Default|GetImpactSurfaceTypes))
          (Default|Fire (Variables|Default|GetWeaponFire)))
        (:then_1
          (Utilities|FlowControl|Delay (Variables|Default|GetBulletTime))
          ;[1 1 1] Spawn and activate Weapon Impact system
          (Utilities|IsValid (Variables|Default|GetWeapon%20Impacts)
            (:Is%20Valid
              _)
            (:Is%20Not%20Valid
              (bind _returnvalue_2 (Game|SpawnActorfromClass "/Game/Effects/Blueprints/B_WeaponImpacts.B_WeaponImpacts_C" (Math|Transform|MakeTransform "0, 0, 0") "Undefined" "OverrideRootScale" 0 5e+02 0))
              (bind _output_get_3 (Variables|Default|SetWeapon%20Impacts _returnvalue_2))
              (Transformation|AttachComponentToComponent _output_get_3 0 "ShootingPoint" "KeepRelative" "KeepRelative" "KeepRelative" true)))
          (Variables|/Game/Effects/Blueprints/B_WeaponImpacts.B_WeaponImpacts_C|SetImpactPositions (Variables|Default|GetWeapon%20Impacts) (Variables|Default|GetImpact%20Positions))
          (Variables|/Game/Effects/Blueprints/B_WeaponImpacts.B_WeaponImpacts_C|SetImpactNormals (Variables|Default|GetWeapon%20Impacts) (Variables|Default|GetImpact%20Normals))
          (Variables|/Game/Effects/Blueprints/B_WeaponImpacts.B_WeaponImpacts_C|SetImpactSurfaceTypes (Variables|Default|GetWeapon%20Impacts) (Variables|Default|GetImpactSurfaceTypes))
          (Variables|/Game/Effects/Blueprints/B_WeaponImpacts.B_WeaponImpacts_C|SetMuzzlePosition (Variables|Default|GetWeapon%20Impacts) (Variables|Default|GetMuzzlePosition))
          (Default|Fire (Variables|Default|GetWeapon%20Impacts)))
        (:then_2
          (Utilities|FlowControl|Delay (Variables|Default|GetBulletTime))
          ;[1 1 1] Spawn and activate Weapon Decal System
          (Utilities|IsValid (Variables|Default|GetWeapon%20Decals)
            (:Is%20Valid
              _)
            (:Is%20Not%20Valid
              (bind _returnvalue_3 (Game|SpawnActorfromClass "/Game/Effects/Blueprints/B_WeaponDecals.B_WeaponDecals_C" (Math|Transform|MakeTransform "0, 0, 0") "Undefined" "OverrideRootScale" 0 0))
              (bind _output_get_4 (Variables|Default|SetWeapon%20Decals _returnvalue_3))
              (Transformation|AttachComponentToComponent _output_get_4 0 "ShootingPoint" "KeepRelative" "KeepRelative" "KeepRelative" true)))
          (Variables|/Game/Effects/Blueprints/B_WeaponDecals.B_WeaponDecals_C|SetImpactPositions (Variables|Default|GetWeapon%20Decals) (Variables|Default|GetImpact%20Positions))
          (Variables|/Game/Effects/Blueprints/B_WeaponDecals.B_WeaponDecals_C|SetImpactNormals (Variables|Default|GetWeapon%20Decals) (Variables|Default|GetImpact%20Normals))
          (Variables|/Game/Effects/Blueprints/B_WeaponDecals.B_WeaponDecals_C|SetImpact%20Surface%20Types (Variables|Default|GetWeapon%20Decals) (Variables|Default|GetImpactSurfaceTypes))
          (Default|Fire (Variables|Default|GetWeapon%20Decals)))
        (:then_3
          (Effects|SpawnEmitterAttached "/Game/Drone/Weapons/Effects/P_AssaultRifle_MF1.P_AssaultRifle_MF1" (Variables|Default|GetWeaponMesh) "ShootingPoint" "0, 0, 0" "0, 0, 0" "0.150000,0.150000,0.150000"))
        (:then_4
          (Audio|PlaySoundatLocation "/Game/Drone/Sounds/Weapon/WeaponFireCue.WeaponFireCue" _output_get "0, 0, 0" 1.0 1.0 0.0 0 0 0 0))
        (:then_5
          (Utilities|FlowControl|Delay (Variables|Default|GetBulletTime))
          (Audio|PlaySoundatLocation "/Game/Drone/Sounds/Weapon/BulletHits/BulletHitWallCue.BulletHitWallCue" [0] "0, 0, 0" 1.0 1.0 0.0 0 0 0 0))))))

(event Custom|ShootBulletMulticast)

(event Custom|DamageWithDelay
  (params (Start :type Vector) (End :type Vector) (Delay :type Float%20%28double-precision%29))
  (Utilities|FlowControl|Delay Delay)
  (bind _asbp_drone_base (Utilities|Casting|CastToBP_DroneBase (Components|GetOwner)))
  (bind _outhit (Collision|LineTraceByChannel Start End "TraceTypeQuery3" false (Utilities|Array|MakeArray (Components|GetOwner) (Default|GetShield _asbp_drone_base)) "None"))
  (bind _asbp_drone_base_2 (Utilities|Casting|CastToBP_DroneBase (.HitActor (Collision|BreakHitResult _outhit)))
    (:then
      (Utilities|Casting|CastToSkeletalMeshComponent (.HitComponent (Collision|BreakHitResult _outhit)))
      (Default|Damage (Variables|/Game/Drone/Blueprints/BP_DroneBase.BP_DroneBase_C|GetBP_IntegralityBase _asbp_drone_base_2) (* (Variables|Default|GetBulletDamage) (Math|Curves|GetFloatValue (Variables|Default|GetDamageCurve) (.Distance (Collision|BreakHitResult _outhit)))))
      (Default|UpdateHealthWidget _asbp_drone_base_2)
      (Default|OnHitMesh (Default|GetShield _asbp_drone_base_2) _outhit))
    (:CastFailed
      (bind _ascannon (Utilities|Casting|CastToCannon (.HitActor (Collision|BreakHitResult _outhit)))
        (:then
          (Utilities|Casting|CastToSphereComponent (.HitComponent (Collision|BreakHitResult _outhit)))
          (Default|Damage (Variables|/Game/Drone/AdditionalObjects/Cannon.Cannon_C|GetBP_IntegralityBase _ascannon) (* (Variables|Default|GetBulletDamage) (Math|Curves|GetFloatValue (Variables|Default|GetDamageCurve) (.Distance (Collision|BreakHitResult _outhit)))))
          (Default|UpdateHealthWidget _ascannon)
          (Development|PrintString (Utilities|String|ToString(Float) (* (Variables|Default|GetBulletDamage) (Math|Curves|GetFloatValue (Variables|Default|GetDamageCurve) (.Distance (Collision|BreakHitResult _outhit)))))))
        (:CastFailed
          (bind _asbp_shield_base (Utilities|Casting|CastToBP_ShieldBase (.HitActor (Collision|BreakHitResult _outhit))))
          (Default|OnShieldHit _asbp_shield_base _outhit (* (* (Variables|Default|GetBulletDamage) (Math|Curves|GetFloatValue (Variables|Default|GetDamageCurve) (.Distance (Collision|BreakHitResult _outhit)))) (Variables|Default|GetDamageShield))))))))

(event EventBeginPlay
  (Utilities|FlowControl|Delay 1.5)
  (CallFunction|DeactivateEvent))

(event Collision|EventActorBeginOverlap
  (params (OtherActor :type Actor%20Object%20Reference)))

(event EventTick
  (params (DeltaSeconds :type Float%20%28single-precision%29))
  (bind _weaponmesh (Variables|Default|GetWeaponMesh))
  (bind _weaponmesh_2 (Variables|Default|GetWeaponMesh))
  (bind _returnvalue (Transformation|GetSocketLocation _weaponmesh "BeginningOfBarrel"))
  (bind _returnvalue_2 (Transformation|GetSocketTransform _weaponmesh_2 "ShootingPoint" "RTS_World"))
  (Variables|Default|SetReloadingTime (+ (Variables|Default|GetReloadingTime) DeltaSeconds))
  (Utilities|FlowControl|Sequence
    (:then_0
      (Networking|SwitchHasAuthority
        (:Remote
          (bind _asbp_drone_base (Utilities|Casting|CastToBP_DroneBase (Components|GetOwner)))
          (bind _outhit (Collision|LineTraceByChannel (.location _returnvalue_2) (+ _returnvalue (* (Math|Vector|GetUnitDirection(Vector) _returnvalue (.location _returnvalue_2)) 5e+04)) "TraceTypeQuery3" false (Utilities|Array|MakeArray (Default|GetShield _asbp_drone_base) (Components|GetOwner)) "None"))
          (Variables|Default|SetOut%20Hit%20Location (.location _outhit))
          (bind _asbp_player_controller (Utilities|Casting|CastToBP_PlayerController (Pawn|GetController _asbp_drone_base)))
          (Variables|/Game/Drone/Blueprints/BP_PlayerController.BP_PlayerController_C|SetAimScreenPosition _asbp_player_controller (.ScreenPosition (Class|GameplayStatics|ProjectWorldtoScreen _asbp_player_controller (.location _outhit) false))))))
    (:then_1
      (if (not (Variables|Default|GetbIsActivated))
        (bind _asbp_drone_base_2 (Utilities|Casting|CastToBP_DroneBase (Components|GetOwner)))
        (Variables|Default|SetAiming (Math|Float|Clamp(Float) (+ -27.0 (* (.pitch (Transformation|GetActorRotation _asbp_drone_base_2)) 1.0)) -5e+01 5e+01))))))

(fn ConstructionScript)

(fn SetSpline
  (params (Spline :type Spline%20Component%20Object%20Reference))
  (Variables|Default|SetSpline Spline))

(fn ChangeAiming
  (params (Value :type Float%20%28double-precision%29))
  (Variables|Default|SetAiming (Math|Float|Clamp(Float) (+ (* Value -0.8) (Variables|Default|GetAiming)) -35.0 3e+01)))

(fn ChangeRotation
  (params (Value :type Float%20%28double-precision%29))
  (Variables|Default|SetRotation (Math|Float|Clamp(Float) (+ (* Value 7.0) (Variables|Default|GetRotation)) -1e+02 1e+02))
  (return (not (CallFunction|IsLimitRotation))))

(fn IsLimitRotation
  (return (> (Math|Float|Absolute(Float) (Variables|Default|GetRotation)) 99.0)))

(fn Damage
  (params (Start :type Vector) (End :type Vector) (Delay :type Float%20%28double-precision%29))
  (bind _output_get (LocalVariables|SetStartLocal Start))
  (bind _output_get_2 (LocalVariables|SetEndLocal End))
  (bind _output_get_3 (LocalVariables|SetDelayLocal Delay))
  (CallFunction|DamagewithDelay _output_get _output_get_2 _output_get_3))