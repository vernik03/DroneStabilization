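; Reinforcement learning manager actor that trains a driving policy, apparently using the Learning Agents plugin.
; BeginPlay sets up the driving interactor, builds the policy on it with the DA_DrivingNetwork asset, then passes both to the RL trainer.
; Tick runs training every frame without reinitializing the policy or critic networks.
; The policy's inference call is left unwired, so the actor only trains.
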(event EventBeginPlay
  (Utilities|FlowControl|Sequence
    (:then_0
      (Class|LearningAgentsInteractor|SetupInteractor (Variables|Default|GetBP_DrivingInteractor)))
    (:then_1
      (Class|LearningAgentsPolicy|SetupPolicy (Variables|Default|GetBP_DrivingPolicy) (Variables|Default|GetBP_DrivingInteractor) (Variables|Default|GetPolicy%20Settings) "/Game/Learning/DA_DrivingNetwork.DA_DrivingNetwork"))
    (:then_2
      (Class|LearningAgentsTrainer|SetupTrainer (Variables|Default|GetBP_DrivingRLTrainer) (Variables|Default|GetBP_DrivingInteractor) (Variables|Default|GetBP_DrivingPolicy) 0 (Variables|Default|GetTrainer%20Settings)))))

(event Collision|EventActorBeginOverlap
  (params (OtherActor :type Actor%20Object%20Reference)))

(event EventTick
  (params (DeltaSeconds :type Float%20%28single-precision%29))
  (Class|LearningAgentsTrainer|RunTraining (Variables|Default|GetBP_DrivingRLTrainer) (Variables|Default|GetTrainer%20Training%20Settings) (Variables|Default|GetTrainer%20Game%20Settings) (Variables|Default|GetTrainer%20Path%20Settings) (Variables|Default|GetCritic%20Settings) false false true))

(fn ConstructionScript)