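; Loot sign actor whose Cylinder animates into place when play begins, growing from nothing to its authored size.
; BeginPlay caches the cylinder's relative height and scale, then plays a Timeline from the start.
; Each update lerps from zero to those cached values, raising and scaling the cylinder while keeping its X/Y position and rotation.
; X and Y scale both use the cached X scale.
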(event EventBeginPlay
  (bind _cylinder (Variables|Default|GetCylinder))
  (bind _cylinder_2 (Variables|Default|GetCylinder))
  (bind _returnvalue (Transformation|GetRelativeTransform _cylinder_2))
  (bind _returnvalue_2 (Transformation|GetRelativeTransform _cylinder))
  (Variables|Default|SetB%20Z (.z (.location _returnvalue_2)))
  (Variables|Default|SetScale%20 (.x (.scale _returnvalue_2)))
  (Variables|Default|Set%20Scale%20Z (.z (.scale _returnvalue_2)))
  (bind _newtrack_0 (Timeline|Timeline PlayFromStart)
    (:Update
      (Transformation|SetRelativeTransform (Variables|Default|GetCylinder) (Math|Transform|MakeTransform (Math|Vector|MakeVector (.x (.location _returnvalue)) (.y (.location _returnvalue)) (.z (Math|Vector|Lerp(Vector) "0, 0, 0" (Math|Vector|MakeVector 0.0 0.0 (Variables|Default|GetB%20Z)) _newtrack_0))) (.rotation _returnvalue) (Math|Vector|MakeVector (.x (Math|Vector|Lerp(Vector) "0, 0, 0" (Math|Vector|MakeVector (Variables|Default|GetScale%20) (Variables|Default|GetScale%20) (Variables|Default|Get%20Scale%20Z)) _newtrack_0)) (.y (Math|Vector|Lerp(Vector) "0, 0, 0" (Math|Vector|MakeVector (Variables|Default|GetScale%20) (Variables|Default|GetScale%20) (Variables|Default|Get%20Scale%20Z)) _newtrack_0)) (.z (Math|Vector|Lerp(Vector) "0, 0, 0" (Math|Vector|MakeVector (Variables|Default|GetScale%20) (Variables|Default|GetScale%20) (Variables|Default|Get%20Scale%20Z)) _newtrack_0)))) false false))))

(event Collision|EventActorBeginOverlap
  (params (OtherActor :type Actor%20Object%20Reference)))

(event EventTick
  (params (DeltaSeconds :type Float%20%28single-precision%29)))

(fn ConstructionScript)