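; Physics-driven pawn for Learning Agents that moves on a thruster and registers itself with any tagged LearningAgentsManager on BeginPlay.
; Tick sets thruster strength from a base value plus scaled ThrustActionPower, which the live event graph only reads.
; ResetToPosition clears motion and teleports back to the recorded start, ignoring its NewLocation input.
; A hand-written Stabilize hover controller and its tuning experiments are left disconnected, alongside debug prints, a start box and a time-dilation key.
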(event Custom|RegisterAgents
  (bind _outactors (Actor|GetAllActorswithTag "LearningAgentsManager"))
  (for _array_element _outactors
    (Utilities|IsValid (Actor|GetComponentbyClass _array_element "/Script/LearningAgents.LearningAgentsManager")
      (:Is%20Valid
        (Class|LearningAgentsManager|AddAgent (Actor|GetComponentbyClass _array_element "/Script/LearningAgents.LearningAgentsManager") self)
        (Variables|Default|SetFoundManager true))))
  (if (not (Variables|Default|GetFoundManager))
    (Development|PrintString "Could not find Learning Agents manager. Did we forget to add one to the scene?")))

(event Collision|EventActorBeginOverlap
  (params (OtherActor :type Actor%20Object%20Reference)))

(event EventTick
  (params (DeltaSeconds :type Float%20%28single-precision%29))
  (bind _thrust_action_power (Variables|Default|GetThrust%20Action%20Power))
  (bind _returnvalue (* _thrust_action_power 2e+02))
  (Variables|/Script/Engine.PhysicsThrusterComponent|SetThrustStrength (Variables|Default|GetPhysicsThruster) (+ (Variables|Default|GetThrust%20Strength%20Base) _returnvalue))
  (Development|PrintString (Utilities|String|ToString(Float) _returnvalue) true false))

(event EventBeginPlay
  (bind _returnvalue (Transformation|GetActorLocation))
  (Variables|Default|SetDeltaPower (Variables|Default|GetDefaultDeltaPower))
  (bind _output_get (Variables|Default|SetStartLocation (Math|Vector|MakeVector (.x _returnvalue) (.y _returnvalue) (.z _returnvalue))))
  (CallFunction|RegisterAgents)
  (Components|Activation|SetActive (Variables|Default|GetPhysicsThruster) true false)
  (Variables|/Script/Engine.PhysicsThrusterComponent|SetThrustStrength (Variables|Default|GetPhysicsThruster) (Variables|Default|GetThrust%20Strength%20Base))
  (Rendering|Debug|DrawDebugBox _output_get (Math|Conversions|ToVector(Float) 6e+01) "(R=0.081892,G=0.331000,B=0.070190,A=1.000000)" "0, 0, 0" 1e+17 3.0))

(event Input|KeyboardEvents|DebugKeyT
  (params (Key :type Key%20Structure :default "None") (ActionValue :type Input%20Action%20Value%20Structure))
  (:Pressed
    (Utilities|Time|SetGlobalTimeDilation 3.0)
    (Development|PrintString "3")))

(fn ConstructionScript)

(fn ResettoPosition
  (params (NewLocation :type Vector))
  (bind _staticmesh (Variables|Default|GetStaticMesh))
  (Physics|SetSimulatePhysics _staticmesh false)
  (Physics|SetPhysicsLinearVelocity _staticmesh "0, 0, 0" false "None")
  (Class|PrimitiveComponent|SetPhysicsAngularVelocityinDegrees _staticmesh "0, 0, 0" false "None") ; Interrupt any angular movement
  (Transformation|SetActorLocation (Variables|Default|GetStartLocation) false true)
  (Transformation|SetActorRotation "0, 0, 0" true)
  (Variables|Default|SetThrust%20Action%20Power 0.0)
  (bind _output_get (Variables|Default|SetThrust%20Strength%20Base (Variables|Default|GetThrust%20Strength%20Base%20Original)))
  (Variables|/Script/Engine.PhysicsThrusterComponent|SetThrustStrength (Variables|Default|GetPhysicsThruster) _output_get)
  (Physics|SetSimulatePhysics (Variables|Default|GetStaticMesh) true))

(fn Stabilize
  (bind _returnvalue (Transformation|GetVelocity))
  (if (Math|Float|NearlyEqual(Float) (.z _returnvalue) 0.0 0.01)
    (bind _output_get (Variables|Default|SetThrust%20Action%20Power 0.0))
    (elif (> (.z _returnvalue) 0.0)
      (Variables|Default|SetThrust%20Action%20Power -1.0)
      (else
        (Variables|Default|SetThrust%20Action%20Power 1.0)))))