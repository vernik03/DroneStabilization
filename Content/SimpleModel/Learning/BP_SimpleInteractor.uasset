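; Learning Agents interactor that defines what each SimplePawn agent observes and how it controls its thrust.
; Observations cover height, vertical velocity, base thrust strength, goal distance and height, plus position and velocity in the pawn's rotation frame.
; Position is measured relative to the agent's previous location, cached in an array indexed by agent ID.
; A single float action is scaled into the pawn's thrust power and printed for debugging.
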(event EventSetupObservations
  (Utilities|FlowControl|Sequence
    (:then_0
      (bind _returnvalue (Class|FloatObservation|AddFloatObservation 0 "ZPositionObservation" 1e+03))
      (Variables|Default|SetZPositionObservation _returnvalue))
    (:then_1
      (bind _returnvalue_2 (Class|FloatObservation|AddFloatObservation 0 "ZVelocityObservation" 1e+03))
      (Variables|Default|SetZVelocityObservation _returnvalue_2))
    (:then_2
      (bind _returnvalue_3 (Class|FloatObservation|AddFloatObservation 0 "PowerObservation" 1e+03))
      (Variables|Default|SetPowerObservation _returnvalue_3))
    (:then_3
      ;[0.06447 1 0.9861] Modified:
      (bind _returnvalue_4 (Class|FloatObservation|AddFloatObservation 0 "DistanceObservation" 1e+03))
      (Variables|Default|SetDistanceObs _returnvalue_4))
    (:then_4
      (bind _returnvalue_5 (Class|FloatObservation|AddFloatObservation 0 "ZGoalObservation" 1e+03))
      (Variables|Default|SetZGoalObservation _returnvalue_5))
    (:then_5
      (bind _returnvalue_6 (Class|PositionObservation|AddPositionObservation 0 "PositionObservation" 1e+03))
      (Variables|Default|SetPositionObservation _returnvalue_6))
    (:then_6
      (bind _returnvalue_7 (Class|VelocityObservation|AddVelocityObservation 0 "VelocityObservation" 2e+02))
      (Variables|Default|SetVelocityObservation _returnvalue_7))))

(event EventSetObservations
  (params (AgentIds :type Array%20of%20Integers))
  (bind _previousposition (Variables|Default|GetPreviousPosition))
  (bind _positionobservation (Variables|Default|GetPositionObservation))
  (for _array_element AgentIds
    (Utilities|FlowControl|Sequence
      (:then_0
        (if (Utilities|Array|IsValidIndex _previousposition _array_element)
          (Class|PositionObservation|SetPositionObservation _positionobservation _array_element (.location (Transformation|GetActorTransform (Class|LearningAgentsManagerComponent|GetAgent _array_element "/Game/SimpleModel/SimplePawn.SimplePawn_C"))) (Utilities|Array|Get(acopy) _previousposition _array_element) (.rotation (Transformation|GetActorTransform (Class|LearningAgentsManagerComponent|GetAgent _array_element "/Game/SimpleModel/SimplePawn.SimplePawn_C"))))
          (Utilities|Array|SetArrayElem (Variables|Default|GetPreviousPosition) _array_element (.location (Transformation|GetActorTransform (Class|LearningAgentsManagerComponent|GetAgent _array_element "/Game/SimpleModel/SimplePawn.SimplePawn_C"))))
          (else
            (Class|PositionObservation|SetPositionObservation _positionobservation _array_element (.location (Transformation|GetActorTransform (Class|LearningAgentsManagerComponent|GetAgent _array_element "/Game/SimpleModel/SimplePawn.SimplePawn_C"))) (.location (Transformation|GetActorTransform (Class|LearningAgentsManagerComponent|GetAgent _array_element "/Game/SimpleModel/SimplePawn.SimplePawn_C"))) (.rotation (Transformation|GetActorTransform (Class|LearningAgentsManagerComponent|GetAgent _array_element "/Game/SimpleModel/SimplePawn.SimplePawn_C"))))
            (Utilities|Array|SetArrayElem (Variables|Default|GetPreviousPosition) _array_element (.location (Transformation|GetActorTransform (Class|LearningAgentsManagerComponent|GetAgent _array_element "/Game/SimpleModel/SimplePawn.SimplePawn_C"))) true))))
      (:then_1
        (Class|VelocityObservation|SetVelocityObservation (Variables|Default|GetVelocityObservation) _array_element (Transformation|GetVelocity (Class|LearningAgentsManagerComponent|GetAgent _array_element "/Game/SimpleModel/SimplePawn.SimplePawn_C")) (Transformation|GetActorRotation (Class|LearningAgentsManagerComponent|GetAgent _array_element "/Game/SimpleModel/SimplePawn.SimplePawn_C"))))
      (:then_4
        (Class|FloatObservation|SetFloatObservation (Variables|Default|GetDistanceObs) _array_element (Math|Vector|Distance(Vector) (Transformation|GetActorLocation (Class|LearningAgentsManagerComponent|GetAgent _array_element "/Game/SimpleModel/SimplePawn.SimplePawn_C")) (Variables|/Game/SimpleModel/SimplePawn.SimplePawn_C|GetGoalLocation (Class|LearningAgentsManagerComponent|GetAgent _array_element "/Game/SimpleModel/SimplePawn.SimplePawn_C")))))
      (:then_5
        (Class|FloatObservation|SetFloatObservation (Variables|Default|GetPowerObservation) _array_element (Variables|/Game/SimpleModel/SimplePawn.SimplePawn_C|GetThrust%20Strength%20Base (Class|LearningAgentsManagerComponent|GetAgent _array_element "/Game/SimpleModel/SimplePawn.SimplePawn_C"))))
      (:then_6
        (Class|FloatObservation|SetFloatObservation (Variables|Default|GetZVelocityObservation) _array_element (.z (Transformation|GetVelocity (Class|LearningAgentsManagerComponent|GetAgent _array_element "/Game/SimpleModel/SimplePawn.SimplePawn_C")))))
      (:then_7
        (Class|FloatObservation|SetFloatObservation (Variables|Default|GetZPositionObservation) _array_element (.z (Transformation|GetActorLocation (Class|LearningAgentsManagerComponent|GetAgent _array_element "/Game/SimpleModel/SimplePawn.SimplePawn_C")))))
      (:then_8
        (Class|FloatObservation|SetFloatObservation (Variables|Default|GetZGoalObservation) _array_element (.z (Variables|/Game/SimpleModel/SimplePawn.SimplePawn_C|GetGoalLocation (Class|LearningAgentsManagerComponent|GetAgent _array_element "/Game/SimpleModel/SimplePawn.SimplePawn_C"))))))))

(event EventSetupActions
  (Utilities|FlowControl|Sequence
    (:then_0
      (bind _returnvalue (Class|FloatAction|AddFloatAction 0 "PowerAction" 2.0))
      (Variables|Default|SetPower _returnvalue))))

(event EventGetActions
  (params (AgentIds :type Array%20of%20Integers))
  (for _array_element AgentIds
    (bind _returnvalue (Class|FloatAction|GetFloatAction (Variables|Default|GetPower) _array_element))
    (bind _output_get (Variables|/Game/SimpleModel/SimplePawn.SimplePawn_C|SetThrust%20Action%20Power (Class|LearningAgentsManagerComponent|GetAgent _array_element "/Game/SimpleModel/SimplePawn.SimplePawn_C") (* _returnvalue 5e+02)))
    (Development|PrintString (Utilities|String|ToString(Float) _output_get) true true "(R=1.000000,G=0.248488,B=0.349717,A=1.000000)")))