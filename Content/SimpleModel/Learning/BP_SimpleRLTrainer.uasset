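; Learning Agents trainer that teaches SimplePawn agents to hold near-zero vertical velocity.
; The velocity reward grows in tiers as absolute Z speed nears zero and turns negative at higher speeds, while a planar position penalty is fed velocity instead of location.
; Excessive vertical speed truncates the episode, and resets return pawns to their StartLocation.
; Goal-location rewards, debug drawing and a long-range completion remain but are disconnected.
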(event EventSetupRewards
  (Utilities|FlowControl|Sequence
    (:then_0
      (bind _returnvalue (Class|ScalarVelocityReward|AddScalarVelocityReward 0 "VelocityReward" 1.0 2e+02))
      (Variables|Default|SetVelocityReward _returnvalue))
    (:then_1
      (bind _returnvalue_2 (Class|PlanarPositionDifferencePenalty|AddPlanarPositionDifferencePenalty 0 "PositionPenalty" 2.0 1e+02 2e+02 "1.000000,0.000000,0.000000" "0.000000,0.000000,1.000000"))
      (Variables|Default|SetPositionPenalty _returnvalue_2))))

(event EventSetRewards
  (params (AgentIds :type Array%20of%20Integers))
  (bind _velocityreward (Variables|Default|GetVelocityReward))
  (for _array_element AgentIds
    (Utilities|FlowControl|Sequence
      (:then_0
        (Class|PlanarPositionDifferencePenalty|SetPlanarPositionDifferencePenalty (Variables|Default|GetPositionPenalty) _array_element (Transformation|GetVelocity (Class|LearningAgentsManagerComponent|GetAgent _array_element "/Game/SimpleModel/SimplePawn.SimplePawn_C")) "0, 0, 0"))
      (:then_1
        (if (< (Math|Float|Absolute(Float) (.z (Transformation|GetVelocity (Class|LearningAgentsManagerComponent|GetAgent _array_element "/Game/SimpleModel/SimplePawn.SimplePawn_C")))) 5e+01)
          (if (< (Math|Float|Absolute(Float) (.z (Transformation|GetVelocity (Class|LearningAgentsManagerComponent|GetAgent _array_element "/Game/SimpleModel/SimplePawn.SimplePawn_C")))) 1.0)
            (if (< (Math|Float|Absolute(Float) (.z (Transformation|GetVelocity (Class|LearningAgentsManagerComponent|GetAgent _array_element "/Game/SimpleModel/SimplePawn.SimplePawn_C")))) 0.01)
              (Class|ScalarVelocityReward|SetScalarVelocityReward _velocityreward _array_element 5.0)
              (else
                (Class|ScalarVelocityReward|SetScalarVelocityReward _velocityreward _array_element 2.0)))
            (else
              (Class|ScalarVelocityReward|SetScalarVelocityReward _velocityreward _array_element (/ 1.0 (Math|Float|Absolute(Float) (.z (Transformation|GetVelocity (Class|LearningAgentsManagerComponent|GetAgent _array_element "/Game/SimpleModel/SimplePawn.SimplePawn_C"))))))))
          (else
            (Class|ScalarVelocityReward|SetScalarVelocityReward _velocityreward _array_element (* (/ (Math|Float|Absolute(Float) (.z (Transformation|GetVelocity (Class|LearningAgentsManagerComponent|GetAgent _array_element "/Game/SimpleModel/SimplePawn.SimplePawn_C")))) 1e+01) -1.0))))))))

(event EventSetupCompletions
  ;[1 1 1] ???
  (Utilities|FlowControl|Sequence
    (:then_1
      (bind _returnvalue (Class|ConditionalCompletion|AddConditionalCompletion 0 "SpeedCompletion" "Truncation"))
      (Variables|Default|SetSpeedCompletion _returnvalue))))

(event EventResetEpisodes
  (params (AgentIds :type Array%20of%20Integers))
  (for _array_element AgentIds
    (Default|ResettoPosition (Class|LearningAgentsManagerComponent|GetAgent _array_element "/Game/SimpleModel/SimplePawn.SimplePawn_C") (Variables|/Game/SimpleModel/SimplePawn.SimplePawn_C|GetStartLocation (Class|LearningAgentsManagerComponent|GetAgent _array_element "/Game/SimpleModel/SimplePawn.SimplePawn_C")))))

(event EventBeginPlay)

(event EventSetCompletions
  (params (AgentIds :type Array%20of%20Integers))
  ;[1 1 1] ???
  (for _array_element AgentIds
    (Utilities|FlowControl|Sequence
      (:then_1
        (Class|ConditionalCompletion|SetConditionalCompletion (Variables|Default|GetSpeedCompletion) _array_element (> (Math|Float|Absolute(Float) (.z (Transformation|GetVelocity (Class|LearningAgentsManagerComponent|GetAgent _array_element "/Game/SimpleModel/SimplePawn.SimplePawn_C")))) 1e+03))))))