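; Learning Agents interactor that defines what a BP_SimplePawn agent observes and the action it can take.
; Observations are a struct of the pawn's location and velocity, both expressed relative to the pawn's own transform, so the location relative to itself carries no positional information.
; The action is a struct with a single Power float, which is written to the pawn's ThrustActionPower when performed.
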(fn SpecifyAgentObservation
  (params (InObservationSchema :type Learning%20Agents%20Observation%20Schema%20Object%20Reference))
  (return (Class|LearningAgentsObservations|SpecifyStructObservation InObservationSchema (Utilities|Map|MakeMap "Location" (Class|LearningAgentsObservations|SpecifyLocationObservation InObservationSchema) "Velocity" (Class|LearningAgentsObservations|SpecifyVelocityObservation InObservationSchema)))))

(fn GatherAgentObservation
  (params (InObservationObject :type Learning%20Agents%20Observation%20Object%20Object%20Reference) (AgentId :type Integer))
  (LocalVariables|SetObsActor (Class|LearningAgentsManagerListener|GetAgent AgentId "/Game/SimpleModel/BP_SimplePawn.BP_SimplePawn_C"))
  (return (Class|LearningAgentsObservations|MakeStructObservation InObservationObject (Utilities|Map|MakeMap "Location" (Class|LearningAgentsObservations|MakeLocationObservation InObservationObject (Transformation|GetActorLocation (LocalVariables|GetObsActor)) (Transformation|GetActorTransform (LocalVariables|GetObsActor)) 1e+04 "LocationObservation" false 0) "Velocity" (Class|LearningAgentsObservations|MakeVelocityObservation InObservationObject (Transformation|GetVelocity (LocalVariables|GetObsActor)) (Transformation|GetActorTransform (LocalVariables|GetObsActor)) 2e+02 "VelocityObservation" true 0)))))

(fn SpecifyAgentAction
  (params (InActionSchema :type Learning%20Agents%20Action%20Schema%20Object%20Reference))
  (return (Class|LearningAgentsActions|SpecifyStructAction InActionSchema (Utilities|Map|MakeMap "Power" (Class|LearningAgentsActions|SpecifyFloatAction InActionSchema "Power")))))

(fn PerformAgentAction
  (params (InActionObject :type Learning%20Agents%20Action%20Object%20Object%20Reference) (InActionObjectElement :type Learning%20Agents%20Action%20Object%20Element%20Structure%20%28by%20ref%29) (AgentId :type Integer))
  (LocalVariables|SetActActor (Class|LearningAgentsManagerListener|GetAgent AgentId "/Game/SimpleModel/BP_SimplePawn.BP_SimplePawn_C"))
  (bind _outelements (Class|LearningAgentsActions|GetStructAction InActionObject InActionObjectElement))
  (Utilities|FlowControl|Sequence
    (:then_0
      (bind _outvalue (Class|LearningAgentsActions|GetFloatAction InActionObject (.Value (Utilities|Map|Find _outelements "Power")) 1.0 "Power" true 0 AgentId))
      (Variables|/Game/SimpleModel/BP_SimplePawn.BP_SimplePawn_C|SetThrust%20Action%20Power (LocalVariables|GetActActor) _outvalue))))