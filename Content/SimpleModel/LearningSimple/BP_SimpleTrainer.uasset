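; Learning Agents trainer Blueprint that defines rewards, episode completion and resets for BP_SimplePawn agents.
; Reward feeds pawn velocity into location helpers with LocationB unset, adding a similarity reward to a penalty past a difference threshold.
; Completion applies a larger threshold to the same velocity, and episode reset returns the pawn to the origin via ResetToPosition.
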(fn GatherAgentReward
  (params (AgentId :type Integer))
  (LocalVariables|SetRewardActor (Class|LearningAgentsManagerListener|GetAgent AgentId "/Game/SimpleModel/BP_SimplePawn.BP_SimplePawn_C"))
  (return (+ (Class|LearningAgentsRewards|MakeRewardfromLocationSimilarity (Transformation|GetVelocity (LocalVariables|GetRewardActor)) "0, 0, 0" 1e+02 1e+01 "LocationSimilarityReward" false 0) (Class|LearningAgentsRewards|MakeRewardonLocationDifferenceAboveThreshold (Transformation|GetVelocity (LocalVariables|GetRewardActor)) "0, 0, 0" 7e+02 -5.0 "LocationDifferenceAboveThresholdReward" true 0))))

(fn GatherAgentCompletion
  (params (AgentId :type Integer))
  (return (Class|LearningAgentsCompletions|MakeCompletiononLocationDifferenceAboveThreshold (Transformation|GetVelocity (Class|LearningAgentsManagerListener|GetAgent AgentId "/Game/SimpleModel/BP_SimplePawn.BP_SimplePawn_C")) "0, 0, 0" 1e+03 "Termination" "LocationDifferenceAboveThresholdCompletion" false 0)))

(fn ResetAgentEpisode
  (params (AgentId :type Integer))
  (Default|ResettoPosition (Class|LearningAgentsManagerListener|GetAgent AgentId "/Game/SimpleModel/BP_SimplePawn.BP_SimplePawn_C") "0, 0, 0"))